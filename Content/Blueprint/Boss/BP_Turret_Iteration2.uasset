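; Boss turret that turns to face the player and fires volleys of bullets.
; After a one-second delay from BeginPlay, Tick snaps its rotation toward the player pawn each frame.
; StartShooting and StopShooting control a looping timer with random start variance; Shoot spawns BP_Bullet_Iteration2 at eight arrow components.
; Dead clears the timer and makes Tick hold zero rotation, leaving the saved initial rotation unused.
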(event `self.ReceiveBeginPlay`
  (set `self.RotationInitial` (`self.K2_GetActorRotation`))
  (`KismetSystemLibrary.Delay` 1.0)
  (set `self.CanRotate` true))

(event `self.ReceiveTick`
  (params (DeltaSeconds :type "Float (single-precision)"))
  (bind _returnvalue (`KismetMathLibrary.Conv_IntToDouble` (`KismetMathLibrary.FFloor` 0.0)))
  (if (`self.CanRotate`)
    (if (`self.IsDead?`)
      (`self.K2_SetActorRotation` (`KismetMathLibrary.MakeRotator` _returnvalue _returnvalue _returnvalue))
      (else
        (`self.K2_SetActorRotation` (`KismetMathLibrary.FindLookAtRotation` (`self.K2_GetActorLocation`) (`self.K2_GetActorLocation` (`GameplayStatics.GetPlayerPawn` 0))))))))

(event `StartShooting`
  (bind _returnvalue (`KismetSystemLibrary.K2_SetTimerDelegate` (`|CreateDelegate` :!event `Shoot`) 0.5 true 0.0 (`KismetMathLibrary.RandomFloatInRange` 0.25 0.75)))
  (set `self.ShootingHandle` _returnvalue))

(event `StopShooting`
  (`KismetSystemLibrary.K2_ClearAndInvalidateTimerHandle` (`self.ShootingHandle`)))

(event `Shoot`
  (for _array_element (`|MakeArray` (`self.Arrow1`) (`self.Arrow2`) (`self.Arrow3`) (`self.Arrow4`) (`self.Arrow5`) (`self.Arrow6`) (`self.Arrow7`) (`self.Arrow8`))
    (`|SpawnActorFromClass` "/Game/Blueprint/Boss/BP_Bullet_Iteration2.BP_Bullet_Iteration2_C" (`KismetMathLibrary.MakeTransform` (`SceneComponent.K2_GetComponentLocation` _array_element) (`SceneComponent.K2_GetComponentRotation` _array_element)) "Undefined" "MultiplyWithRoot" null null)))

(event `Dead`
  (set `self.IsDead?` true)
  (`KismetSystemLibrary.K2_ClearAndInvalidateTimerHandle` (`self.ShootingHandle`)))

(fn `UserConstructionScript`)