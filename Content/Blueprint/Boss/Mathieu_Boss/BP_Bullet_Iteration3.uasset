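; BP_Bullet_Iteration3 is a boss bullet that damages the player's X-wing on contact.
; One second after BeginPlay, its static mesh switches to overlapping all collision channels.
; The Box overlap casts the other actor to BP_Xwing, applies fixed damage, prints the amount and destroys the bullet.
; Other actors are ignored, and the mesh's own overlap event is empty.
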(event `self.ReceiveBeginPlay`
  (`KismetSystemLibrary.Delay` 1.0)
  (`PrimitiveComponent.SetCollisionResponseToAllChannels` (`self.StaticMesh`) "ECR_Overlap"))

(event `self.StaticMesh.OnComponentBeginOverlap`
  (params (OverlappedComponent :type "PrimitiveComponent Object Reference") (OtherActor :type "Actor Object Reference") (OtherComp :type "PrimitiveComponent Object Reference") (OtherBodyIndex :type Integer) (bFromSweep :type Boolean) (SweepResult :type "HitResult Structure (by ref)")))

(event `self.Box.OnComponentBeginOverlap`
  (params (OverlappedComponent :type "PrimitiveComponent Object Reference") (OtherActor :type "Actor Object Reference") (OtherComp :type "PrimitiveComponent Object Reference") (OtherBodyIndex :type Integer) (bFromSweep :type Boolean) (SweepResult :type "HitResult Structure (by ref)"))
  (bind _asbp_xwing (cast `/Game/Blueprint/XwingPlayer/BP_Xwing` OtherActor))
  (bind _returnvalue (`GameplayStatics.ApplyDamage` _asbp_xwing 10.0 null self))
  (`KismetSystemLibrary.PrintString` (`KismetStringLibrary.Concat_StrStr` "Damage given : " (`KismetStringLibrary.Conv_DoubleToString` _returnvalue)))
  (`self.K2_DestroyActor`))

(fn `UserConstructionScript`)