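; Boss actor that fights in phases ("Paterns"), emerging from nest actors with turrets attached to its body sockets.
; Tick drives constant-speed moves to nest targets with camera shake and force feedback, switched on the current phase.
; In phase one, damage kills random turrets at health intervals, then low health starts the nest-to-nest phase two.
; An inter-phase event raises a shield, stops turret fire and triggers trash-mob spawners; phase three is an empty stub.
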(event `self.ReceiveBeginPlay`
  ;[1 1 1] General
  (`KismetSystemLibrary.K2_SetTimerDelegate` (`|CreateDelegate` :!event `StartPatern1`) 5.0)
  (bind _returnvalue (`|CreateWidget` "/Game/Mathis/UI/HUD/WI_HUD.WI_HUD_C"))
  (set `self.HUD ref` _returnvalue))

(event `self.ReceiveTick`
  (params (DeltaSeconds :type "Float (single-precision)"))
  ;[1 1 1] General
  (`KismetSystemLibrary.PrintString` (`KismetStringLibrary.Concat_StrStr` "Boss Health : " (`KismetStringLibrary.Conv_DoubleToString` (`self.Health`))) true true (struct :`R` 1.0 :`G` 0.543455 :`A` 1.0) 0.0)
  (switch `int` (`self.Patern?`)
    (:`0`
      (`self.RiseAnim`)
      (`KismetSystemLibrary.PrintString` (`KismetStringLibrary.Conv_DoubleToString` (`self.Health`)) true true (struct :`G` 0.66 :`B` 1.0 :`A` 1.0) 0.0))
    (:`1`
      (if (`self.CanMove?`)
        (`self.GoToNextNest`)))))

(event `Shoot`
  ;[1 1 1] General
  (for _array_element (`self.TurretRefArray`)
    (`/Game/Blueprint/Boss/Mathieu_Boss/BP_Turret.StartShooting` _array_element)))

(event `self.ReceiveAnyDamage`
  (params (Damage :type "Float (single-precision)") (DamageType :type "DamageType Object Reference") (InstigatedBy :type "Controller Object Reference") (DamageCauser :type "Actor Object Reference"))
  ;[1 1 1] General
  (set `self.Health` (`KismetMathLibrary.FClamp` (- (`self.Health`) 10.0) 0.0 (`self.MaxHealth`)))
  (switch `int` (`self.Patern?`)
    (:`0`
      (`self.Patern1HealthCheck`))))

(event `StartPatern1`
  ;[1 1 1] General
  (bind _outactors (`GameplayStatics.GetAllActorsOfClass` "/Game/Blueprint/Boss/Mathieu_Boss/BP_NestExit.BP_NestExit_C"))
  (bind _output_get (set `self.NestExitRef` (`KismetArrayLibrary.Array_Random` _outactors)))
  (set `self.TargetLocation` (`SceneComponent.K2_GetComponentLocation` (`/Game/Blueprint/Boss/Mathieu_Boss/BP_NestExit.Exit` _output_get)))
  (`self.K2_SetActorLocationAndRotation` (`self.K2_GetActorLocation` _output_get) (`KismetMathLibrary.MakeRotator` (+ (.roll (`self.K2_GetActorRotation` _output_get)) 90.0) (.pitch (`self.K2_GetActorRotation` _output_get)) (.yaw (`self.K2_GetActorRotation` _output_get))))
  (`self.SpawnTurretMacro`)
  (`self.RiseMyChildRise`))

(event `RiseMyChildRise`
  ;[0.4048 0 1] Patern 1
  (set `self.CanRise?` true)
  (`KismetSystemLibrary.K2_SetTimerDelegate` (`|CreateDelegate` :!event `Shoot`) 0.5 false 10.0)
  (`AudioComponent.Play` (`self.Audio`) 0.0))

(event `StartPatern2`
  ;[0 1 0.04712] Patern 2
  (bind _outactors (`GameplayStatics.GetAllActorsOfClass` "/Game/Blueprint/Boss/Mathieu_Boss/BP_NestPatern2_Start.BP_NestPatern2_Start_C"))
  (bind _output_get (set `self.NestPatern2` (`KismetArrayLibrary.Array_Random` _outactors)))
  (set `self.TargetLocation` (`SceneComponent.K2_GetComponentLocation` (`/Game/Blueprint/Boss/Mathieu_Boss/BP_NestPatern2_End.EndPoint` (`/Game/Blueprint/Boss/Mathieu_Boss/BP_NestPatern2_Start.BP_Patern2_End` _output_get))))
  (`self.K2_SetActorLocationAndRotation` (`self.K2_GetActorLocation` _output_get) (`KismetMathLibrary.MakeRotator` (+ (.roll (`self.K2_GetActorRotation` _output_get)) 90.0) (.pitch (`self.K2_GetActorRotation` _output_get)) (.yaw (`self.K2_GetActorRotation` _output_get))))
  (set `self.CanMove?` true))

(event `GoToNextNest`
  (bind _returnvalue (`self.K2_GetActorLocation`))
  (bind _targetlocation (`self.TargetLocation`))
  ;[0 1 0.04712] Patern 2
  (`self.K2_SetActorLocation` (`KismetMathLibrary.VInterpTo_Constant` _returnvalue _targetlocation (`GameplayStatics.GetWorldDeltaSeconds`) 7500.0))
  (if (!= _returnvalue _targetlocation :`ErrorTolerance` 1.0)
    (`GameplayStatics.PlayWorldCameraShake` "/Game/Blueprint/Boss/Mathieu_Boss/MONCAMERASHAKE.MONCAMERASHAKE_C" _returnvalue 0.0 10000000.0)
    (`ActorComponent.Activate` (`self.ForceFeedback`) false)
    (else
      (`ActorComponent.Deactivate` (`self.ForceFeedback`))
      (set `self.CanMove?` false)
      (`KismetSystemLibrary.K2_SetTimerDelegate` (`|CreateDelegate` :!event `StartPatern2`) 2.5))))

(event `RiseAnim`
  (bind _returnvalue (`self.K2_GetActorLocation`))
  (bind _targetlocation (`self.TargetLocation`))
  ;[0.4048 0 1] Patern 1
  (if (`self.CanRise?`)
    (`self.K2_SetActorLocation` (`KismetMathLibrary.VInterpTo_Constant` _returnvalue _targetlocation (`GameplayStatics.GetWorldDeltaSeconds`) 100000.0))
    (if (!= _returnvalue _targetlocation :`ErrorTolerance` 1.0)
      (`GameplayStatics.PlayWorldCameraShake` "/Game/Blueprint/Boss/Mathieu_Boss/MONCAMERASHAKE.MONCAMERASHAKE_C" _returnvalue 0.0 10000000.0)
      (`ActorComponent.Activate` (`self.ForceFeedback`) false)
      (else
        (`ActorComponent.Deactivate` (`self.ForceFeedback`))
        (set `self.CanRise?` false)))))

(event `CheckHealthPatern2`
  ;[0 1 0.04712] Patern 2
  (if (not (!= (`self.Health`) 0.0))
    (`self.K2_TeleportTo` (-10000.0 -10000.0 -10000.0))
    (set `self.CanMove?` false)))

(event `Patern1HealthCheck`
  ;[0.4048 0 1] Patern 1
  (if (== (mod (`self.Health`) 1000.0) (mod (`self.MaxHealth`) 1000.0))
    (bind _output_get (set `self.TurretDead` (`KismetArrayLibrary.Array_Random` (`self.TurretRefArray`))))
    (`/Game/Blueprint/Boss/Mathieu_Boss/BP_Turret.Dead` _output_get)
    (if (< (`self.Health`) 10.0)
      (`self.DeathPatern1`))))

(event `DeathPatern2`
  ;[0 1 0.04712] Patern 2
  (set `self.Patern?` 2)
  (`KismetSystemLibrary.K2_SetTimerDelegate` (`|CreateDelegate` :!event `InterPatern`) 2.0))

(event `DeathPatern1`
  ;[0.4048 0 1] Patern 1
  (bind _output_get (set `self.Patern?` 1))
  (`KismetSystemLibrary.PrintString` (`KismetStringLibrary.Concat_StrStr` "Patern set is : " (`KismetStringLibrary.Conv_IntToString` _output_get)))
  (`KismetSystemLibrary.K2_SetTimerDelegate` (`|CreateDelegate` :!event `InterPatern`) 2.0)
  (`self.StartPatern2`))

(event `StartPatern 3`)

(event `InterPatern`
  (`SceneComponent.SetHiddenInGame` (`self.Shield`) false false)
  (for _array_element (`self.TurretRefArray`)
    (`/Game/Blueprint/Boss/Mathieu_Boss/BP_Turret.StopShooting` _array_element))
  (`PrimitiveComponent.SetCollisionResponseToAllChannels` (`self.Shield`) "ECR_Block")
  (`KismetSystemLibrary.PrintString` "Shield Collission")
  (bind _outactors (`GameplayStatics.GetAllActorsOfClass` "/Game/Blueprint/IA_Trashmob/BP_Spawn_AI_Trashmob.BP_Spawn_AI_Trashmob_C"))
  (for _array_element_2 _outactors
    (`/Game/Blueprint/IA_Trashmob/BP_Spawn_AI_Trashmob.AI_Spawn_By_Boss` _array_element_2))
  (`KismetSystemLibrary.PrintString` "Finish spawn IA"))

(fn `SpawnTurret`
  (returns (Array :type "Array of /Game/Blueprint/Boss/Mathieu_Boss/BP_Turret Object Reference"))
  (bind _returnvalue (`|SpawnActorFromClass` "/Game/Blueprint/Boss/Mathieu_Boss/BP_Turret.BP_Turret_C" (`KismetMathLibrary.MakeTransform` (0.0 0.0 0.0)) "Undefined" "MultiplyWithRoot" null null))
  (`self.K2_AttachToActor` _returnvalue self "Turret1" "SnapToTarget" "KeepRelative" "KeepRelative" true)
  (bind _returnvalue_2 (`|SpawnActorFromClass` "/Game/Blueprint/Boss/Mathieu_Boss/BP_Turret.BP_Turret_C" (`KismetMathLibrary.MakeTransform` (0.0 0.0 0.0)) "Undefined" "MultiplyWithRoot" null null))
  (`self.K2_AttachToActor` _returnvalue_2 self "Turret2" "SnapToTarget" "KeepRelative" "KeepRelative" true)
  (bind _returnvalue_3 (`|SpawnActorFromClass` "/Game/Blueprint/Boss/Mathieu_Boss/BP_Turret.BP_Turret_C" (`KismetMathLibrary.MakeTransform` (0.0 0.0 0.0)) "Undefined" "MultiplyWithRoot" null null))
  (`self.K2_AttachToActor` _returnvalue_3 self "Turret3" "SnapToTarget" "KeepRelative" "KeepRelative" true)
  (bind _returnvalue_4 (`|SpawnActorFromClass` "/Game/Blueprint/Boss/Mathieu_Boss/BP_Turret.BP_Turret_C" (`KismetMathLibrary.MakeTransform` (0.0 0.0 0.0)) "Undefined" "MultiplyWithRoot" null null))
  (`self.K2_AttachToActor` _returnvalue_4 self "Turret4" "SnapToTarget" "KeepRelative" "KeepRelative" true)
  (bind _returnvalue_5 (`|SpawnActorFromClass` "/Game/Blueprint/Boss/Mathieu_Boss/BP_Turret.BP_Turret_C" (`KismetMathLibrary.MakeTransform` (0.0 0.0 0.0)) "Undefined" "MultiplyWithRoot" null null))
  (`self.K2_AttachToActor` _returnvalue_5 self "Turret5" "SnapToTarget" "KeepRelative" "KeepRelative" true)
  (bind _returnvalue_6 (`|SpawnActorFromClass` "/Game/Blueprint/Boss/Mathieu_Boss/BP_Turret.BP_Turret_C" (`KismetMathLibrary.MakeTransform` (0.0 0.0 0.0)) "Undefined" "MultiplyWithRoot" null null))
  (`self.K2_AttachToActor` _returnvalue_6 self "Turret6" "SnapToTarget" "KeepRelative" "KeepRelative" true)
  (bind _returnvalue_7 (`|SpawnActorFromClass` "/Game/Blueprint/Boss/Mathieu_Boss/BP_Turret.BP_Turret_C" (`KismetMathLibrary.MakeTransform` (0.0 0.0 0.0)) "Undefined" "MultiplyWithRoot" null null))
  (`self.K2_AttachToActor` _returnvalue_7 self "Turret7" "SnapToTarget" "KeepRelative" "KeepRelative" true)
  (bind _returnvalue_8 (`|SpawnActorFromClass` "/Game/Blueprint/Boss/Mathieu_Boss/BP_Turret.BP_Turret_C" (`KismetMathLibrary.MakeTransform` (0.0 0.0 0.0)) "Undefined" "MultiplyWithRoot" null null))
  (`self.K2_AttachToActor` _returnvalue_8 self "Turret8" "SnapToTarget" "KeepRelative" "KeepRelative" true)
  (return (`|MakeArray` _returnvalue _returnvalue_2 _returnvalue_3 _returnvalue_4 _returnvalue_5 _returnvalue_6 _returnvalue_7 _returnvalue_8)))

(fn `UserConstructionScript`)