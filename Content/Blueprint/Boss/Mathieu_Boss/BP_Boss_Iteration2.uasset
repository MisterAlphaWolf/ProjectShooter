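; Multi-phase boss that emerges from random nests, shaking camera and gamepad as it moves.
; Pattern 1 rises from a nest exit with turrets attached to body sockets; pattern 2 travels toward a nest end point, both interpolated on Tick.
; Interphases advance the pattern, raise an invulnerability shield, stop turrets and spawn trash mobs on a looping timer, then restore health.
; Pattern 3 is an empty stub; debug prints remain.
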(event `self.ReceiveBeginPlay`
  ;[1 1 1] Begin play
  (bind _returnvalue (`GameplayStatics.GetActorOfClass` "/Game/Blueprint/IA_Trashmob/BP_Spawn_AI_Trashmob.BP_Spawn_AI_Trashmob_C"))
  (set `self.Spawn trashmob ref` _returnvalue))

(event `Paterne change`
  ;[1 1 1] Paterne change
  (switch `int` (`self.Patern?`)
    (:`0`
      (`KismetSystemLibrary.K2_SetTimerDelegate` (`|CreateDelegate` :!event `StartPatern1`) 5.0))
    (:`1`
      (`KismetSystemLibrary.K2_SetTimerDelegate` (`|CreateDelegate` :!event `StartPatern2`) 5.0))))

(event `self.ReceiveTick`
  (params (DeltaSeconds :type "Float (single-precision)"))
  ;[1 1 1] General
  (`KismetSystemLibrary.PrintString` (`KismetStringLibrary.Concat_StrStr` "Boss Health : " (`KismetStringLibrary.Conv_DoubleToString` (`self.Health`))) true true (struct :`R` 1.0 :`G` 0.543455 :`A` 1.0) 0.0)
  (switch `int` (`self.Patern?`)
    (:`0`
      (`self.RiseAnim`))
    (:`1`
      (if (`self.CanMove?`)
        (`self.GoToNextNest`)))))

(event `Shoot`
  ;[1 1 1] General
  (for _array_element (`self.TurretRefArray`)
    (`/Game/Blueprint/Boss/Mathieu_Boss/BP_Turret_Iteration2.UpdateTurret` _array_element)
    (`/Game/Blueprint/Boss/Mathieu_Boss/BP_Turret_Iteration2.StartShooting` _array_element)))

(event `Interphase`
  (bind _shield (`self.Shield`))
  ;[1 1 1] Interphase
  (set `self.Patern?` (+ (`self.Patern?`) 1))
  (set `self.Can take damage ?` false)
  (`SceneComponent.SetVisibility` _shield true false)
  (`PrimitiveComponent.SetCollisionEnabled` _shield "QueryAndPhysics")
  (for _array_element (`self.TurretRefArray`)
    (`/Game/Blueprint/Boss/Mathieu_Boss/BP_Turret_Iteration2.StopShooting` _array_element))
  (bind _returnvalue (`KismetSystemLibrary.K2_SetTimerDelegate` (delegate `Spawn Ennemi`) 0.25 true))
  (set `self.Event spawn ennemi` _returnvalue))

(event `self.ReceiveAnyDamage`
  (params (Damage :type "Float (single-precision)") (DamageType :type "DamageType Object Reference") (InstigatedBy :type "Controller Object Reference") (DamageCauser :type "Actor Object Reference"))
  ;[1 1 1] General
  (if (`self.Can take damage ?`)
    (bind _output_get (set `self.Health` (`KismetMathLibrary.FClamp` (- (`self.Health`) Damage) 0.0 (`self.MaxHealth`))))
    (if (<= _output_get 0.0)
      (switch `int` (`self.Patern?`)
        (:`0`
          (`self.Patern1HealthCheck`))))))

(event `Spawn Ennemi`
  (bind _nbtrashmob (`self.NBtrashmob`))
  ;[1 1 1] Interphase
  (if (> _nbtrashmob 0)
    (`/Engine/EditorBlueprintResources/StandardMacros.DecrementInt` _nbtrashmob
      (:`  `
        (`/Game/Blueprint/IA_Trashmob/BP_Spawn_AI_Trashmob.AI_Spawn_By_Boss` (`self.Spawn trashmob ref`))))
    (else
      (`KismetSystemLibrary.K2_ClearAndInvalidateTimerHandle` (`self.Event spawn ennemi`))
      (`KismetSystemLibrary.Delay` (`self.Duree interphase`))
      (`self.Fin interphase`))))

(event `Fin interphase`
  (bind _shield (`self.Shield`))
  ;[1 1 1] Interphase
  (set `self.Can take damage ?` true)
  (`SceneComponent.SetVisibility` _shield false false)
  (`PrimitiveComponent.SetCollisionEnabled` _shield "NoCollision")
  (set `self.Health` (`self.MaxHealth`))
  (`KismetSystemLibrary.K2_SetTimerDelegate` (`|CreateDelegate` :!event `Paterne change`) 5.0))

(event `StartPatern1`
  ;[1 1 1] General
  (bind _output_get (set `self.NestExitRef` (`KismetArrayLibrary.Array_Random` (`self.NestExist`))))
  (set `self.TargetLocation` (`SceneComponent.K2_GetComponentLocation` (`/Game/Blueprint/Boss/Mathieu_Boss/BP_NestExit.Exit` _output_get)))
  (`self.K2_SetActorLocationAndRotation` (`self.K2_GetActorLocation` _output_get) (`SceneComponent.K2_GetComponentRotation` (`/Game/Blueprint/Boss/Mathieu_Boss/BP_NestExit.Arrow` _output_get)))
  (`self.SpawnTurretMacro`)
  (`self.RiseMyChildRise`))

(event `RiseMyChildRise`
  ;[0.4048 0 1] Patern 1
  (set `self.CanRise?` true)
  (`KismetSystemLibrary.K2_SetTimerDelegate` (`|CreateDelegate` :!event `Shoot`) 0.5 false 10.0)
  (`AudioComponent.Play` (`self.Audio`) 0.0))

(event `StartPatern2`
  ;[0 1 0.04712] Patern 2
  (`KismetSystemLibrary.PrintString` "Start Patern 2")
  (bind _output_get (set `self.NestPatern2` (`KismetArrayLibrary.Array_Random` (`self.NestPatern`))))
  (set `self.TargetLocation` (`SceneComponent.K2_GetComponentLocation` (`/Game/Blueprint/Boss/Mathieu_Boss/BP_NestPatern2_End.EndPoint` (`/Game/Blueprint/Boss/Mathieu_Boss/BP_NestPatern2_Start.BP_Patern2_End` _output_get))))
  (`self.K2_SetActorLocationAndRotation` (`self.K2_GetActorLocation` _output_get) (`KismetMathLibrary.MakeRotator` (+ (.roll (`self.K2_GetActorRotation` _output_get)) 90.0) (.pitch (`self.K2_GetActorRotation` _output_get)) (.yaw (`self.K2_GetActorRotation` _output_get))))
  (set `self.CanMove?` true))

(event `GoToNextNest`
  (bind _returnvalue (`self.K2_GetActorLocation`))
  (bind _targetlocation (`self.TargetLocation`))
  ;[0 1 0.04712] Patern 2
  (`self.K2_SetActorLocation` (`KismetMathLibrary.VInterpTo_Constant` _returnvalue _targetlocation (`GameplayStatics.GetWorldDeltaSeconds`) 7500.0))
  (if (!= _returnvalue _targetlocation :`ErrorTolerance` 1.0)
    (`GameplayStatics.PlayWorldCameraShake` "/Game/Blueprint/Boss/Mathieu_Boss/MONCAMERASHAKE.MONCAMERASHAKE_C" _returnvalue 0.0 10000000.0)
    (`ActorComponent.Activate` (`self.ForceFeedback`) false)
    (else
      (`ActorComponent.Deactivate` (`self.ForceFeedback`))
      (set `self.CanMove?` false)
      (`KismetSystemLibrary.K2_SetTimerDelegate` (`|CreateDelegate` :!event `StartPatern2`) 2.5))))

(event `RiseAnim`
  (bind _returnvalue (`self.K2_GetActorLocation`))
  (bind _targetlocation (`self.TargetLocation`))
  ;[0.4048 0 1] Patern 1
  (if (`self.CanRise?`)
    (`self.K2_SetActorLocation` (`KismetMathLibrary.VInterpTo_Constant` _returnvalue _targetlocation (`GameplayStatics.GetWorldDeltaSeconds`) 50000.0))
    (if (!= _returnvalue _targetlocation :`ErrorTolerance` 1.0)
      (`GameplayStatics.PlayWorldCameraShake` "/Game/Blueprint/Boss/Mathieu_Boss/MONCAMERASHAKE.MONCAMERASHAKE_C" _returnvalue 0.0 10000000.0)
      (`ActorComponent.Activate` (`self.ForceFeedback`) false)
      (else
        (`ActorComponent.Deactivate` (`self.ForceFeedback`))
        (set `self.CanRise?` false)))))

(event `CheckHealthPatern2`
  ;[0 1 0.04712] Patern 2
  (if (not (!= (`self.Health`) 0.0))
    (`self.K2_TeleportTo` (-10000.0 -10000.0 -10000.0))
    (set `self.CanMove?` false)))

(event `Patern1HealthCheck`
  (bind _returnvalue (mod (`self.Health`) 1000.0))
  ;[0.4048 0 1] Patern 1
  (`KismetSystemLibrary.PrintString` (`KismetStringLibrary.Conv_DoubleToString` _returnvalue) true true (struct :`R` 1.0 :`G` 0.701195 :`A` 1.0))
  (if (== _returnvalue (mod (`self.MaxHealth`) 1000.0))
    (bind _output_get (set `self.TurretDead` (`KismetArrayLibrary.Array_Random` (`self.TurretRefArray`))))
    (`/Game/Blueprint/Boss/Mathieu_Boss/BP_Turret_Iteration2.Dead` _output_get)
    (`KismetArrayLibrary.Array_RemoveItem` (`self.TurretRefArray`) _output_get)
    (if (< (`self.Health`) 10.0)
      (`self.DeathPatern1`))))

(event `DeathPatern2`
  ;[0 1 0.04712] Patern 2
  (set `self.Patern?` 2)
  (`KismetSystemLibrary.K2_SetTimerDelegate` (`|CreateDelegate` :!event `Interphase`) 2.0))

(event `DeathPatern1`
  ;[0.4048 0 1] Patern 1
  (`KismetSystemLibrary.K2_SetTimerDelegate` (`|CreateDelegate` :!event `Interphase`) 2.0))

(event `StartPatern 3`)

(fn `SpawnTurret`
  (returns (Array :type "Array of /Game/Blueprint/Boss/Mathieu_Boss/BP_Turret Object Reference"))
  (bind _returnvalue (`|SpawnActorFromClass` "/Game/Blueprint/Boss/Mathieu_Boss/BP_Turret.BP_Turret_C" (`KismetMathLibrary.MakeTransform` (0.0 0.0 0.0)) "Undefined" "MultiplyWithRoot" null null))
  (`self.K2_AttachToActor` _returnvalue self "Turret1" "SnapToTarget" "KeepRelative" "KeepRelative" true)
  (bind _returnvalue_2 (`|SpawnActorFromClass` "/Game/Blueprint/Boss/Mathieu_Boss/BP_Turret.BP_Turret_C" (`KismetMathLibrary.MakeTransform` (0.0 0.0 0.0)) "Undefined" "MultiplyWithRoot" null null))
  (`self.K2_AttachToActor` _returnvalue_2 self "Turret2" "SnapToTarget" "KeepRelative" "KeepRelative" true)
  (bind _returnvalue_3 (`|SpawnActorFromClass` "/Game/Blueprint/Boss/Mathieu_Boss/BP_Turret.BP_Turret_C" (`KismetMathLibrary.MakeTransform` (0.0 0.0 0.0)) "Undefined" "MultiplyWithRoot" null null))
  (`self.K2_AttachToActor` _returnvalue_3 self "Turret3" "SnapToTarget" "KeepRelative" "KeepRelative" true)
  (bind _returnvalue_4 (`|SpawnActorFromClass` "/Game/Blueprint/Boss/Mathieu_Boss/BP_Turret.BP_Turret_C" (`KismetMathLibrary.MakeTransform` (0.0 0.0 0.0)) "Undefined" "MultiplyWithRoot" null null))
  (`self.K2_AttachToActor` _returnvalue_4 self "Turret4" "SnapToTarget" "KeepRelative" "KeepRelative" true)
  (bind _returnvalue_5 (`|SpawnActorFromClass` "/Game/Blueprint/Boss/Mathieu_Boss/BP_Turret.BP_Turret_C" (`KismetMathLibrary.MakeTransform` (0.0 0.0 0.0)) "Undefined" "MultiplyWithRoot" null null))
  (`self.K2_AttachToActor` _returnvalue_5 self "Turret5" "SnapToTarget" "KeepRelative" "KeepRelative" true)
  (bind _returnvalue_6 (`|SpawnActorFromClass` "/Game/Blueprint/Boss/Mathieu_Boss/BP_Turret.BP_Turret_C" (`KismetMathLibrary.MakeTransform` (0.0 0.0 0.0)) "Undefined" "MultiplyWithRoot" null null))
  (`self.K2_AttachToActor` _returnvalue_6 self "Turret6" "SnapToTarget" "KeepRelative" "KeepRelative" true)
  (bind _returnvalue_7 (`|SpawnActorFromClass` "/Game/Blueprint/Boss/Mathieu_Boss/BP_Turret.BP_Turret_C" (`KismetMathLibrary.MakeTransform` (0.0 0.0 0.0)) "Undefined" "MultiplyWithRoot" null null))
  (`self.K2_AttachToActor` _returnvalue_7 self "Turret7" "SnapToTarget" "KeepRelative" "KeepRelative" true)
  (bind _returnvalue_8 (`|SpawnActorFromClass` "/Game/Blueprint/Boss/Mathieu_Boss/BP_Turret.BP_Turret_C" (`KismetMathLibrary.MakeTransform` (0.0 0.0 0.0)) "Undefined" "MultiplyWithRoot" null null))
  (`self.K2_AttachToActor` _returnvalue_8 self "Turret8" "SnapToTarget" "KeepRelative" "KeepRelative" true)
  (return (`|MakeArray` _returnvalue _returnvalue_2 _returnvalue_3 _returnvalue_4 _returnvalue_5 _returnvalue_6 _returnvalue_7 _returnvalue_8)))

(fn `UserConstructionScript`
  (bind _scale_boss_largeur (`self.Scale boss largeur`))
  (bind _scale_boss_longeur (`self.Scale boss longeur`))
  (bind _returnvalue (+ _scale_boss_largeur 100.0))
  (bind _returnvalue_2 (/ _scale_boss_largeur 800.0))
  (`SceneComponent.SetWorldScale3D` (`self.Boss Body`) (`KismetMathLibrary.MakeVector` _scale_boss_largeur _scale_boss_largeur _scale_boss_longeur))
  (`SceneComponent.SetWorldScale3D` (`self.Shield`) (`KismetMathLibrary.MakeVector` _returnvalue _returnvalue (* _scale_boss_longeur 1.45)))
  (`SceneComponent.SetWorldScale3D` (`self.MouthPartIteration2_2`) (`KismetMathLibrary.MakeVector` _returnvalue_2 _returnvalue_2 _returnvalue_2))
  (`SceneComponent.SetWorldScale3D` (`self.MouthPartIteration2`) (`KismetMathLibrary.MakeVector` _returnvalue_2 _returnvalue_2 _returnvalue_2))
  (`SceneComponent.SetWorldScale3D` (`self.MouthPartIteration2_3`) (`KismetMathLibrary.MakeVector` _returnvalue_2 _returnvalue_2 _returnvalue_2))
  (`SceneComponent.SetWorldScale3D` (`self.MouthPartIteration2_4`) (`KismetMathLibrary.MakeVector` _returnvalue_2 _returnvalue_2 _returnvalue_2)))