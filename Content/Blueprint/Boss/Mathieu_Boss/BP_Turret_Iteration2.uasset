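; Boss turret that aims at a point far ahead of the player's X-wing and fires bullet volleys.
; Once updated, it rotates every tick, limiting each axis with a tolerance around its initial rotation.
; A looping, start-jittered timer drives shooting, with a delayed-loop macro spawning bullets from eight arrows in shuffled order.
; Death stops the timer and zeroes rotation; the construction script scales it from the boss's width.
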(event `self.ReceiveBeginPlay`
  (bind _asbp_xwing (cast `/Game/Blueprint/XwingPlayer/BP_Xwing` (`GameplayStatics.GetPlayerPawn` 0)))
  (set `self.As BP Xwing` _asbp_xwing))

(event `UpdateTurret`
  (set `self.CanRotate` true))

(event `self.ReceiveTick`
  (params (DeltaSeconds :type "Float (single-precision)"))
  (bind _as_bp_xwing (`self.As BP Xwing`))
  (bind _returnvalue (`KismetMathLibrary.Conv_IntToDouble` (`KismetMathLibrary.FFloor` 0.0)))
  (if (`self.CanRotate`)
    (if (`self.IsDead?`)
      (`self.K2_SetActorRotation` (`KismetMathLibrary.MakeRotator` _returnvalue _returnvalue _returnvalue))
      (else
        (`self.K2_SetActorRotation` (`KismetMathLibrary.MakeRotator` (`self.GetAxisRotation` (.roll (`KismetMathLibrary.FindLookAtRotation` (`self.K2_GetActorLocation`) (+ (`self.K2_GetActorLocation` _as_bp_xwing) (* (`self.GetActorForwardVector` _as_bp_xwing) 10000.0)))) (.roll (`self.RotationInitial`)) (`self.ToleranceRotation`)) (`self.GetAxisRotation` (.pitch (`KismetMathLibrary.FindLookAtRotation` (`self.K2_GetActorLocation`) (+ (`self.K2_GetActorLocation` _as_bp_xwing) (* (`self.GetActorForwardVector` _as_bp_xwing) 10000.0)))) (.pitch (`self.RotationInitial`)) (`self.ToleranceRotation`)) (`self.GetAxisRotation` (.yaw (`KismetMathLibrary.FindLookAtRotation` (`self.K2_GetActorLocation`) (+ (`self.K2_GetActorLocation` _as_bp_xwing) (* (`self.GetActorForwardVector` _as_bp_xwing) 10000.0)))) (.yaw (`self.RotationInitial`)) (`self.ToleranceRotation`))))
        (`KismetSystemLibrary.PrintString` (`KismetStringLibrary.Concat_StrStr` "Tourret Rotation : " (`KismetStringLibrary.Conv_RotatorToString` (`self.RotationInitial`)) " at " (`KismetSystemLibrary.GetDisplayName` self)) true true (struct :`R` 1.0 :`G` 0.195013 :`B` 0.335047 :`A` 1.0) 0.0)))))

(event `StartShooting`
  (bind _returnvalue (`KismetSystemLibrary.K2_SetTimerDelegate` (`|CreateDelegate` :!event `Shoot`) 2.5 true 0.0 (`KismetMathLibrary.RandomFloatInRange` 0.25 0.75)))
  (set `self.ShootingHandle` _returnvalue))

(event `Shoot`
  (bind _array_element (`self.CustomLoop` (`|MakeArray` (`self.Arrow1`) (`self.Arrow2`) (`self.Arrow3`) (`self.Arrow4`) (`self.Arrow5`) (`self.Arrow6`) (`self.Arrow7`) (`self.Arrow8`)) 0.125)
    (:`Loop Body`
      (`|SpawnActorFromClass` "/Game/Blueprint/Boss/Mathieu_Boss/BP_Bullet_Iteration3.BP_Bullet_Iteration3_C" (`KismetMathLibrary.MakeTransform` (`SceneComponent.K2_GetComponentLocation` _array_element) (`SceneComponent.K2_GetComponentRotation` _array_element)) "Undefined" "MultiplyWithRoot" null null))))

(event `StopShooting`
  (`KismetSystemLibrary.K2_ClearAndInvalidateTimerHandle` (`self.ShootingHandle`)))

(event `Dead`
  (set `self.IsDead?` true)
  (`KismetSystemLibrary.K2_ClearAndInvalidateTimerHandle` (`self.ShootingHandle`)))

(fn `GetAxisRotation`
  (params (CurrentAxis :type "Float (double-precision)") (InitAxis :type "Float (double-precision)") (AxisDelta :type "Float (double-precision)" :default 45.0))
  (returns (FinalAxis :type "Float (double-precision)"))
  (bind _returnvalue (`KismetMathLibrary.Abs` CurrentAxis))
  (bind _returnvalue_2 (`KismetMathLibrary.Abs` InitAxis))
  (bind _returnvalue_3 (+ _returnvalue_2 AxisDelta))
  (bind _returnvalue_4 (- _returnvalue_2 AxisDelta))
  (return (`KismetMathLibrary.SelectFloat` _returnvalue_3 (`KismetMathLibrary.SelectFloat` _returnvalue_4 CurrentAxis (<= _returnvalue _returnvalue_4)) (>= _returnvalue _returnvalue_3))))

(fn `UserConstructionScript`
  (bind _returnvalue (`GameplayStatics.GetActorOfClass` "/Game/Blueprint/Boss/Mathieu_Boss/BP_Boss_Iteration2.BP_Boss_Iteration2_C"))
  (bind _returnvalue_2 (/ (`/Game/Blueprint/Boss/Mathieu_Boss/BP_Boss_Iteration2.Scale boss largeur` _returnvalue) 500.0))
  (`SceneComponent.SetWorldScale3D` (`self.Scene`) (`KismetMathLibrary.MakeVector` _returnvalue_2 _returnvalue_2 _returnvalue_2)))