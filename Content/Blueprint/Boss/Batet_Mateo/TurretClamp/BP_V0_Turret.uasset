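; BP_V0_Turret is a destructible boss turret that tracks and shoots at the player pawn.
; Tick turns it at constant speed toward the player, clamping pitch and yaw around its starting rotation.
; While shooting is enabled, a forward line trace starts a looping bullet-spawn timer when the path is clear or hits the player, and stops it when blocked.
; At zero HP it stops firing, hides, disables collision and damages BossRef.
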(event `self.ReceiveBeginPlay`
  (set `self.InitRotator` (`self.K2_GetActorRotation`))
  (set `self.HP` (`self.HP_Max`)))

(event `Fire`
  (`|SpawnActorFromClass` "/Game/Blueprint/Boss/Mathieu_Boss/BP_Bullet_Iteration3.BP_Bullet_Iteration3_C" (`SceneComponent.K2_GetComponentToWorld` (`self.FireDirection`)) "AlwaysSpawn" "MultiplyWithRoot" null null))

(event `HandleShoot`
  (params (CanShoot :type Boolean))
  (if CanShoot
    (set `self.CanShoot` true)
    (else
      (set `self.CanShoot` false)
      (`KismetSystemLibrary.K2_ClearAndInvalidateTimerHandle` (`self.FireTimer`))
      (set `self.IsShooting` false))))

(event `self.ReceiveTick`
  (params (DeltaSeconds :type "Float (single-precision)"))
  (bind _returnvalue (`self.K2_GetActorLocation`))
  (bind _initrotator_roll (`KismetMathLibrary.BreakRotator` (`self.InitRotator`)))
  (bind (_initrotator_roll_2 _initrotator_pitch _initrotator_yaw) (`KismetMathLibrary.BreakRotator` (`self.InitRotator`)))
  (bind _angleclamp (`self.AngleClamp`))
  (bind _angleclamp_2 (`self.AngleClamp`))
  (bind (_returnvalue_roll _returnvalue_pitch _returnvalue_yaw) (`KismetMathLibrary.BreakRotator` (`KismetMathLibrary.FindLookAtRotation` (`self.K2_GetActorLocation`) (`self.K2_GetActorLocation` (`GameplayStatics.GetPlayerPawn` 0)))))
  (`self.K2_SetActorRotation` (`KismetMathLibrary.RInterpTo_Constant` (`self.K2_GetActorRotation`) (`KismetMathLibrary.MakeRotator` _initrotator_roll (`KismetMathLibrary.ClampAngle` _returnvalue_pitch (- _initrotator_pitch _angleclamp) (+ _initrotator_pitch _angleclamp)) (`KismetMathLibrary.ClampAngle` _returnvalue_yaw (- _initrotator_yaw _angleclamp_2) (+ _initrotator_yaw _angleclamp_2))) (`GameplayStatics.GetWorldDeltaSeconds`) (`self.SpeedRotation`)))
  (if (`self.CanShoot`)
    (bind (_outhit _returnvalue_2) (`KismetSystemLibrary.LineTraceSingle` _returnvalue (+ _returnvalue (* (`SceneComponent.GetForwardVector` (`self.FireDirection`)) (`self.FireRange`))) "TraceTypeQuery4"))
    (if (or (== (`.HitActor` (`GameplayStatics.BreakHitResult` _outhit)) (`GameplayStatics.GetPlayerPawn` 0)) (not _returnvalue_2))
      (if (not (`self.IsShooting`))
        (bind _returnvalue_3 (`KismetSystemLibrary.K2_SetTimerDelegate` (delegate `Fire`) (`self.TImerBetweenProjectile`) true))
        (set `self.FireTimer` _returnvalue_3)
        (set `self.IsShooting` true))
      (elif (`self.IsShooting`)
        (`KismetSystemLibrary.K2_ClearAndInvalidateTimerHandle` (`self.FireTimer`))
        (set `self.IsShooting` false)))))

(event `self.ReceiveAnyDamage`
  (params (Damage :type "Float (single-precision)") (DamageType :type "DamageType Object Reference") (InstigatedBy :type "Controller Object Reference") (DamageCauser :type "Actor Object Reference"))
  (set `self.HP` (- (`self.HP`) Damage))
  (if (<= (`self.HP`) 0.0)
    (`self.HandleShoot` false)
    (`PrimitiveComponent.SetCollisionEnabled` (`self.Turret2iteration`) "NoCollision")
    (`self.SetActorHiddenInGame` true)
    (bind _bossref (`self.BossRef`)
      (:`then`
        (`GameplayStatics.ApplyDamage` _bossref (`self.DeathDamage`) null self))
      (:`else`))))

(fn `UserConstructionScript`)