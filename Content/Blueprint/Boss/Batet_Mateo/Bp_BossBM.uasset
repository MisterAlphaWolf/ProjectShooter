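; Boss actor that moves between spots, carrying a ring of turrets spawned and attached at its arrow components.
; A timeline moves it vertically at a spot drawn from a refilling random pool; reversing it leads to the next spot.
; Turrets fire via tick toggling once the forward move ends.
; Half health triggers phase two, where it keeps relocating with turrets off while stamina remains; zero health only prints "Dead".
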(event `self.ReceiveAnyDamage`
  (params (Damage :type "Float (single-precision)") (DamageType :type "DamageType Object Reference") (InstigatedBy :type "Controller Object Reference") (DamageCauser :type "Actor Object Reference"))
  (bind _output_get (set `self.Hp` (- (`self.Hp`) Damage)))
  (if (<= _output_get 0.0)
    (`KismetSystemLibrary.PrintString` "Dead")
    (elif (<= (`self.Hp`) (/ (`self.HpMax`) 2.0))
      (set `self.PhaseNumber` 2)
      (`self.EndSpot`))))

(event `ChooseRandomSpot`
  (bind _tabtemp (`self.TabTemp`))
  (bind _outitem (`KismetArrayLibrary.Array_Random` _tabtemp))
  (if (`KismetArrayLibrary.Array_IsEmpty` (`self.TabTemp`))
    (set `self.TabTemp` (`self.TabSpot`)))
  (bind _output_get (set `self.ChooseSpotCurrent` _outitem))
  (`KismetArrayLibrary.Array_RemoveItem` _tabtemp _outitem)
  (bind (_direction _lerp) (`Timeline|Up/Down` :!via `PlayFromStart` :!label _label)
    (:`Update`
      (bind (_returnvalue_x _returnvalue_y _returnvalue_z) (`KismetMathLibrary.BreakVector` (`self.K2_GetActorLocation` _output_get)))
      (`self.K2_SetActorLocation` (`KismetMathLibrary.VLerp` (`self.K2_GetActorLocation` _output_get) (`KismetMathLibrary.MakeVector` _returnvalue_x _returnvalue_y (+ _returnvalue_z 10000.0)) _lerp)))
    (:`Finished`
      (switch `ETimelineDirection` _direction
        (:`Forward`
          (if (== (`self.PhaseNumber`) 2)
            (if (<= (`self.Stamina`) 0.0)
              (`self.ShootTuret` true)
              (else
                (`self.EndSpot`)
                (`self.ShootTuret` false)))
            (else
              (`self.ShootTuret` true))))
        (:`Backward`
          (`self.ChooseRandomSpot`))))))

(event `EndSpot`
  (goto _label :!via `Reverse`))

(event `ShootTuret`
  (params (`StopShoot?` :type Boolean))
  (for _array_element (`self.TuretTab`)
    (`self.SetActorTickEnabled` _array_element `StopShoot?`)))

(event `self.ReceiveBeginPlay`
  (for _array_element (`|MakeArray` (`self.Arrow17`) (`self.Arrow2`) (`self.Arrow6`) (`self.Arrow3`) (`self.Arrow4`) (`self.Arrow5`) (`self.Arrow25`) (`self.Arrow26`) (`self.Arrow27`) (`self.Arrow24`) (`self.Arrow28`) (`self.Arrow29`) (`self.Arrow30`) (`self.Arrow15`) (`self.Arrow16`) (`self.Arrow1`) (`self.Arrow18`) (`self.Arrow19`) (`self.Arrow23`) (`self.Arrow20`) (`self.Arrow21`) (`self.Arrow22`) (`self.Arrow7`) (`self.Arrow8`) (`self.Arrow9`) (`self.Arrow10`) (`self.Arrow11`) (`self.Arrow12`) (`self.Arrow13`) (`self.Arrow14`))
    (bind (_returnvalue_location _returnvalue_rotation) (`KismetMathLibrary.BreakTransform` (`SceneComponent.K2_GetComponentToWorld` _array_element)))
    (bind _returnvalue (`|SpawnActorFromClass` "/Game/Blueprint/Boss/Batet_Mateo/BP_V0_Turret.BP_V0_Turret_C" (`KismetMathLibrary.MakeTransform` _returnvalue_location _returnvalue_rotation (0.1 0.1 0.1)) "AlwaysSpawn" "MultiplyWithRoot" null null))
    (`KismetArrayLibrary.Array_AddUnique` (`self.TuretTab`) _returnvalue)
    (`self.K2_AttachToComponent` _returnvalue _array_element "None" "SnapToTarget" "SnapToTarget" "KeepRelative" true))
  (`self.ShootTuret` false)
  (`self.ChooseRandomSpot`))

(fn `UserConstructionScript`)