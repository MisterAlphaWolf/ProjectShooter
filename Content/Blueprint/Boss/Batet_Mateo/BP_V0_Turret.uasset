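; Turret actor, apparently a first version for a boss, that turns to face the first player's pawn; it has no firing logic.
; Each Tick rotates the whole actor toward the look-at rotation with RInterpToConstant at SpeedRotation.
; The construction script derives pitch and yaw limits around the initial rotation, but the clamp nodes using them are unconnected, so rotation is unrestricted.
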(event `self.ReceiveTick`
  (params (DeltaSeconds :type "Float (single-precision)"))
  (`self.K2_SetActorRotation` (`KismetMathLibrary.MakeRotator` (.roll (`KismetMathLibrary.RInterpTo_Constant` (`self.K2_GetActorRotation`) (`KismetMathLibrary.FindLookAtRotation` (`self.K2_GetActorLocation`) (`self.K2_GetActorLocation` (`GameplayStatics.GetPlayerPawn` 0))) (`GameplayStatics.GetWorldDeltaSeconds`) (`self.SpeedRotation`))) (.pitch (`KismetMathLibrary.RInterpTo_Constant` (`self.K2_GetActorRotation`) (`KismetMathLibrary.FindLookAtRotation` (`self.K2_GetActorLocation`) (`self.K2_GetActorLocation` (`GameplayStatics.GetPlayerPawn` 0))) (`GameplayStatics.GetWorldDeltaSeconds`) (`self.SpeedRotation`))) (.yaw (`KismetMathLibrary.RInterpTo_Constant` (`self.K2_GetActorRotation`) (`KismetMathLibrary.FindLookAtRotation` (`self.K2_GetActorLocation`) (`self.K2_GetActorLocation` (`GameplayStatics.GetPlayerPawn` 0))) (`GameplayStatics.GetWorldDeltaSeconds`) (`self.SpeedRotation`))))))

(fn `UserConstructionScript`
  (bind (_returnvalue_roll _returnvalue_pitch _returnvalue_yaw) (`KismetMathLibrary.BreakRotator` (`self.K2_GetActorRotation`)))
  (set `self.MinAnglePitch` (- _returnvalue_pitch 70.0))
  (set `self.MaxAnglePitch` (+ _returnvalue_pitch 70.0))
  (set `self.MinAngleYaw` (- _returnvalue_yaw 70.0))
  (set `self.MaxAngleYaw` (+ _returnvalue_yaw 70.0)))