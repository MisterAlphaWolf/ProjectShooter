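; Boss turret Blueprint that tracks the player's X-wing and fires bullets on a repeating timer.
; After a short delay from BeginPlay, Tick rotates the whole actor to face the first BP_Xwing found.
; StartShooting begins a looping timer with randomized start variance, and Shoot spawns BP_Bullet at the Arrow component's transform.
; Dead stops the timer, activates two Niagara smoke effects and makes Tick hold rotation at zero.
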(event `self.ReceiveBeginPlay`
  (set `self.RotationInitial` (`self.K2_GetActorRotation`))
  (`KismetSystemLibrary.Delay` 1.0)
  (set `self.CanRotate` true)
  (bind _returnvalue (`GameplayStatics.GetActorOfClass` "/Game/XwingPlayer/BP_Xwing.BP_Xwing_C"))
  (set `self.Player_Ref` _returnvalue))

(event `self.ReceiveTick`
  (params (DeltaSeconds :type "Float (single-precision)"))
  (bind _returnvalue (`KismetMathLibrary.Conv_IntToDouble` (`KismetMathLibrary.FFloor` 0.0)))
  (if (`self.CanRotate`)
    (if (`self.IsDead?`)
      (`self.K2_SetActorRotation` (`KismetMathLibrary.MakeRotator` _returnvalue _returnvalue _returnvalue))
      (else
        (`self.K2_SetActorRotation` (`KismetMathLibrary.FindLookAtRotation` (`self.K2_GetActorLocation`) (`self.K2_GetActorLocation` (`self.Player_Ref`))))))))

(event `StartShooting`
  (bind _returnvalue (`KismetSystemLibrary.K2_SetTimerDelegate` (`|CreateDelegate` :!event `Shoot`) 0.25 true 0.0 (`KismetMathLibrary.RandomFloatInRange` 0.25 0.75)))
  (set `self.ShootingHandle` _returnvalue))

(event `Shoot`
  (bind _arrow (`self.Arrow`))
  (`|SpawnActorFromClass` "/Game/Blueprint/Boss/BP_Bullet.BP_Bullet_C" (`KismetMathLibrary.MakeTransform` (`SceneComponent.K2_GetComponentLocation` _arrow) (`SceneComponent.K2_GetComponentRotation` _arrow)) "Undefined" "MultiplyWithRoot" null null))

(event `Dead`
  (set `self.IsDead?` true)
  (`KismetSystemLibrary.K2_ClearAndInvalidateTimerHandle` (`self.ShootingHandle`))
  (`ActorComponent.Activate` (`self.NS_SmokeRock`) false)
  (`ActorComponent.Activate` (`self.NS_SmokeRock1`) false))

(fn `UserConstructionScript`)