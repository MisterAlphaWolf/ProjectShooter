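; Trashmob enemy ship AI that chases the BP_Xwing player at a player-scaled speed and dies to BP_Projectile damage.
; Tick drives an enum movement state: follow, move forward, or dodge.
; A sphere trace detects range, and looping timers toggle dodging, which steers along the player's front or back spline chosen by facing dot product.
; Bullet-firing timer setup and random weak-point selection are disconnected; construction hides all weak points.
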(event `self.ReceiveBeginPlay`
  ;[0 0 0] Set_Ref_&_Variables
  (bind _returnvalue (`GameplayStatics.GetActorOfClass` "/Game/XwingPlayer/BP_Xwing.BP_Xwing_C"))
  (set `self.Player_Ref` _returnvalue)
  (set `self.AI_Is_In_Range_Of_Player` false)
  (set `self.E_AI_Movement` "NewEnumerator0")
  (if (not (`KismetSystemLibrary.K2_IsTimerActiveHandle` (`self.Is_Undodge_Timer_Event_Ref`)))
    (bind _returnvalue_2 (`KismetSystemLibrary.K2_SetTimerDelegate` (`|CreateDelegate` :!event `UnDodge_Player_Event  `) 0.5 true))
    (set `self.Is_Undodge_Timer_Event_Ref` _returnvalue_2)))

(event `self.ReceiveTick`
  (params (DeltaSeconds :type "Float (single-precision)"))
  (`|ExecutionSequence`
    (:`then_0`
      (`self.Distance_To_Player`)
      ;[1 1 0] AI_Switch_Movement
      (switch `/Game/Blueprint/IA_Trashmob/BP/E_AI_Movement` (`self.E_AI_Movement`)
        (:`NewEnumerator0`
          (`self.AI_Rotate_To_Player`)
          (`self.AI_Move_Forward`)
          (`self.AI_Can_Shoot_??`))
        (:`NewEnumerator1`
          (`self.AI_Move_Forward`)
          (`self.AI_Can_Shoot_??`))
        (:`NewEnumerator4`
          (`self.FollowSpline`)
          (`self.AI_Move_Forward`)
          (`self.AI_Can_Shoot_??`))
        (:`NewEnumerator2`
          (`self.AI_Rotate_To_Player`)
          (`self.AI_Can_Shoot_??`))
        (:`NewEnumerator3`
          (`self.AI_Rotate_To_Player`)
          (`self.AI_Can_Shoot_??`))))
    (:`then_1`
      (`self.Debug`))))

(event `Distance_To_Player`
  ;[0.02985 1 0.9502] Get/Set_Distance_To_Player_&_Set_AI_Speed_Modifier
  (set `self.Distance_AI_To_Player` (`self.GetDistanceTo` (`self.Player_Ref`)))
  (set `self.Speed_Multiply` (* (`/Game/XwingPlayer/BP_Xwing.Current forward speed` (`self.Player_Ref`)) 2.0)))

(event `self.ReceiveAnyDamage`
  (params (Damage :type "Float (single-precision)") (DamageType :type "DamageType Object Reference") (InstigatedBy :type "Controller Object Reference") (DamageCauser :type "Actor Object Reference"))
  ;[1 0 0] Kill_AI_When_Player_Bullet_Touch_Them
  (cast `/Game/XwingPlayer/BP_Projectile` DamageCauser)
  (`self.K2_DestroyActor`))

(event `Debug`
  ;[1 1 1] Debug
  (`KismetSystemLibrary.PrintText` (`|FormatText` "Player Speed : {A} \nDistance AI To Player: {B} \nAI Speed Multiply : {C} \nE AI Movement : {D} \nAI Is In Range Of Player : {E}" (`/Game/XwingPlayer/BP_Xwing.Current forward speed` (`self.Player_Ref`)) (`self.Distance_AI_To_Player`) (`self.Speed_Multiply`) (`|GetEnumeratorNameAsString` (`self.E_AI_Movement`)) (`self.AI_Is_In_Range_Of_Player`)) true true (struct :`R` 0.035046 :`G` 1.0 :`A` 1.0) 0.0))

(event `Dodge_Player_Event`
  (`self.Player_Ref`
    (:`then`
      (if (`self.AI_Is_In_Range_Of_Player`)
        (set `self.PlayerSplineRef` (`self.Get_Spline_Ref`))
        (set `self.E_AI_Movement` "NewEnumerator4")
        (`KismetSystemLibrary.K2_PauseTimerHandle` (`self.Event_Shoot`))))
    (:`else`)))

(event `FollowSpline`
  (bind _playersplineref (`self.PlayerSplineRef`)
    (:`then`
      (bind _output_get (set `self.SplineLocTarget` (`SplineComponent.FindLocationClosestToWorldLocation` _playersplineref (+ (`self.K2_GetActorLocation`) (* (`self.GetActorForwardVector`) 400.0)) "World")))
      (bind _output_get_2 (set `self.AI_New_Rotation` (`KismetMathLibrary.RInterpTo_Constant` (`self.K2_GetActorRotation`) (`KismetMathLibrary.FindLookAtRotation` (`self.K2_GetActorLocation`) _output_get) (`GameplayStatics.GetWorldDeltaSeconds`) 100.0)))
      (`self.K2_SetActorRotation` _output_get_2)
      (if (== (`SplineComponent.GetDistanceAlongSplineAtLocation` (`self.PlayerSplineRef`) (`self.SplineLocTarget`) "World") 0.0)
        (set `self.E_AI_Movement` "NewEnumerator1")))
    (:`else`)))

(event `UnDodge_Player_Event`
  (`self.Player_Ref`
    (:`then`
      (if (not (`self.AI_Is_In_Range_Of_Player`))
        (set `self.E_AI_Movement` "NewEnumerator0")
        (`KismetSystemLibrary.K2_UnPauseTimerHandle` (`self.Event_Shoot`))))
    (:`else`)))

(event `AI_Can_Shoot_??`
  (bind _returnvalue (`SceneComponent.K2_GetComponentLocation` (`self.AI_Trashmob`)))
  ;[1 0.4353 0] AI_Range_To_See_Player
  (bind (_outhit _returnvalue_2) (`KismetSystemLibrary.SphereTraceSingle` :`Start` _returnvalue :`End` _returnvalue :`Radius` 5000.0 :`TraceChannel` "TraceTypeQuery3" :`DrawDebugType` "ForOneFrame"))
  (bind _output_get (set `self.AI_Is_In_Range_Of_Player` _returnvalue_2))
  (if _output_get
    (cast `/Game/XwingPlayer/BP_Xwing` (`.HitActor` (`GameplayStatics.BreakHitResult` _outhit))
      (:`then`
        (if (not (`KismetSystemLibrary.K2_IsTimerActiveHandle` (`self.Is_Dodge_Timer_Event_Ref`)))
          (bind _returnvalue_3 (`KismetSystemLibrary.K2_SetTimerDelegate` (`|CreateDelegate` :!event `Dodge_Player_Event`) 0.5 true))
          (set `self.Is_Dodge_Timer_Event_Ref` _returnvalue_3)))
      (:`CastFailed`
        (`KismetSystemLibrary.K2_PauseTimerHandle` (`self.Event_Shoot`) :!label _label)))
    (else
      (goto _label))))

(event `AI_Shoot`
  (bind _shootstart (`self.ShootStart`))
  ;[1 0.4353 0] Shoot_Event
  (`|SpawnActorFromClass` "/Game/Blueprint/Boss/BP_Bullet.BP_Bullet_C" (`KismetMathLibrary.MakeTransform` (`SceneComponent.K2_GetComponentLocation` _shootstart) (`KismetMathLibrary.Conv_VectorToRotator` (`SceneComponent.GetForwardVector` _shootstart))) "AlwaysSpawn" "MultiplyWithRoot" null null))

(fn `AI_Move_Forward`
  (`self.AddMovementInput` (* (`KismetMathLibrary.GetForwardVector` (`self.K2_GetActorRotation`)) (`self.Speed_Multiply`))))

(fn `AI_Rotate_To_Player`
  (bind _output_get (set `self.AI_New_Rotation` (`KismetMathLibrary.RInterpTo_Constant` (`self.K2_GetActorRotation`) (`KismetMathLibrary.FindLookAtRotation` (`self.K2_GetActorLocation`) (`self.K2_GetActorLocation` (`self.Player_Ref`))) (`GameplayStatics.GetWorldDeltaSeconds`) 100.0)))
  (`self.K2_SetActorRotation` _output_get))

(fn `AI_Speed_Modifier_To_Catch_Player`
  ;[0 0 0] PAS TOUCHER !!!!
)

(fn `Get_Spline_Ref`
  (returns (ReturnValue :type "SplineComponent Object Reference"))
  (bind _player_ref (`self.Player_Ref`))
  (return (select `bool` (> (`KismetMathLibrary.Dot_VectorVector` (`self.GetActorForwardVector` (`self.Player_Ref`)) (`self.GetActorForwardVector`)) 0.0) :`false` (`/Game/XwingPlayer/BP_Xwing.Front_Spline` _player_ref) :`true` (`/Game/XwingPlayer/BP_Xwing.Back_Spline` _player_ref))))

(fn `UserConstructionScript`
  (bind _weakpoint_01 (`self.WeakPoint_01`))
  ;[0 0 0] Random_WeakPoint
  ;
  ; NE PAS TOUCHER
  (`SceneComponent.SetVisibility` _weakpoint_01 false false)
  (`SceneComponent.SetVisibility` (`self.WeakPoint_02`) false false)
  (`SceneComponent.SetVisibility` (`self.WeakPoint_03`) false false)
  (`PrimitiveComponent.SetCollisionEnabled` _weakpoint_01 "NoCollision")
  (`PrimitiveComponent.SetCollisionEnabled` (`self.WeakPoint_02`) "NoCollision")
  (`PrimitiveComponent.SetCollisionEnabled` (`self.WeakPoint_03`) "NoCollision")
  (`SceneComponent.SetHiddenInGame` _weakpoint_01 true false)
  (`SceneComponent.SetHiddenInGame` (`self.WeakPoint_02`) true false)
  (`SceneComponent.SetHiddenInGame` (`self.WeakPoint_03`) true false))