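; Base trashmob enemy AI that targets the player X-wing and dies on any damage.
; Tick switches on a movement enum (follow, forward, spline dodge, rotate-only debug) and sphere-traces for the player, but BeginPlay sets Debug mode.
; A looping distance timer drives shooting, which reuses bullets from a pool of pre-placed actors.
; Dodge timers, random weak-point selection and catch-up speed logic are disconnected, and construction hides all weak points.
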(event `self.ReceiveBeginPlay`
  ;[0 0 0] Set_Ref_&_Variables
  (bind _returnvalue (`GameplayStatics.GetActorOfClass` "/Game/XwingPlayer/BP_Xwing.BP_Xwing_C"))
  (set `self.Player_Ref` _returnvalue)
  (bind _outactors (`GameplayStatics.GetAllActorsOfClass` "/Game/Blueprint/IA_Trashmob/BP/BP_AI_Bullet.BP_AI_Bullet_C"))
  (set `self.AI_Bullet_Ref` _outactors)
  (set `self.AI_Is_In_Range_Of_Player` false)
  (set `self.Speed_Multiply` (* (`/Game/XwingPlayer/BP_Xwing.Current forward speed` (`self.Player_Ref`)) 2.0))
  (bind _returnvalue_2 (`KismetSystemLibrary.K2_SetTimer` null "Get/Set_Distance_To_Player_Call_Shoot_Event_Function" 0.2 true))
  (set `self.Distance_To_Player_Timer_Event_Ref` _returnvalue_2)
  (if (not (`KismetSystemLibrary.K2_IsTimerActiveHandle` (`self.Debug_Print_Timer_Function_Ref`)))
    (bind _returnvalue_3 (`KismetSystemLibrary.K2_SetTimer` null "Debug_Print_Function" 0.015 true))
    (set `self.Debug_Print_Timer_Function_Ref` _returnvalue_3)
    (bind _returnvalue_4 (`GameplayStatics.GetActorOfClass` "/Game/Blueprint/IA_Trashmob/BP/BP_AI_Trashmob_Child.BP_AI_Trashmob_Child_C"))
    (set `self.AI_Trashmob_Child_Ref` _returnvalue_4)
    (set `self.E_AI_Movement` "NewEnumerator2")))

(event `self.ReceiveTick`
  (params (DeltaSeconds :type "Float (single-precision)"))
  (`|ExecutionSequence`
    (:`then_0`
      ;[1 1 0] AI_Switch_Movement
      (switch `/Game/Blueprint/IA_Trashmob/BP/E_AI_Master_Movement` (`self.E_AI_Movement`)
        (:`NewEnumerator0`
          (`self.AI_Rotate_To_Player_Function`)
          (`self.AI_Move_Forward_Function`)
          (`self.AI_Range_To_See_Player`))
        (:`NewEnumerator1`
          (`self.AI_Move_Forward_Function`)
          (`self.AI_Range_To_See_Player`))
        (:`NewEnumerator4`
          (`self.Follow_Spline_Function`)
          (`self.AI_Move_Forward_Function`)
          (`self.AI_Range_To_See_Player`))
        (:`NewEnumerator2`
          (`self.AI_Rotate_To_Player_Function`)
          (`self.AI_Range_To_See_Player`))
        (:`NewEnumerator5`
          (`self.AI_Rotate_To_Player_Function`)
          (`self.AI_Range_To_See_Player`))))))

(event `self.ReceiveAnyDamage`
  (params (Damage :type "Float (single-precision)") (DamageType :type "DamageType Object Reference") (InstigatedBy :type "Controller Object Reference") (DamageCauser :type "Actor Object Reference"))
  ;[1 0 0] Kill_AI_When_Player_Bullet_Touch_Them
  (`self.K2_DestroyActor`))

(event `self.OptimizationProxy.OnChangeWave`
  (params (NewWave :type "EOptimizationWave Enum" :default "Invisible"))
  (set `self.E_On_Change_Wave` NewWave))

(event `AI_Range_To_See_Player`
  (bind _returnvalue (`SceneComponent.K2_GetComponentLocation` (`self.AI_Trashmob`)))
  ;[1 0.4353 0] AI_Range_To_See_Player
  (bind (_outhit _returnvalue_2) (`KismetSystemLibrary.SphereTraceSingle` _returnvalue _returnvalue 5000.0 "TraceTypeQuery3"))
  (bind _output_get (set `self.AI_Is_In_Range_Of_Player` _returnvalue_2))
  (if _output_get
    (cast `/Game/XwingPlayer/BP_Xwing` (`.HitActor` (`GameplayStatics.BreakHitResult` _outhit))
      (:`then`
        (if (not (`KismetSystemLibrary.K2_IsTimerActiveHandle` (`self.Dodge_Timer_Function_Ref`)))
          _))
      (:`CastFailed`
        (`KismetSystemLibrary.K2_PauseTimerHandle` (`self.Event_Shoot`) :!label _label)))
    (else
      (goto _label))))

(event `realoadBullet`
  (bind _output (`|GetArrayItem` (`self.AI_Bullet_Ref`) (`self.NBullet`)))
  ;[1 0.4353 0] Shoot_Event
  (if (not (`/Game/Blueprint/IA_Trashmob/BP/BP_AI_Bullet.isUse` _output)) :!label _label_2
    (bind _output_get (set `self.bullet` _output))
    (set `/Game/Blueprint/IA_Trashmob/BP/BP_AI_Bullet.isUse` true _output_get)
    (`/Game/Blueprint/IA_Trashmob/BP/BP_AI_Bullet.Spawn_Bullet_Function` _output)
    (`self.K2_SetActorLocationAndRotation` (`self.bullet`) (`SceneComponent.K2_GetComponentLocation` (`self.Arrow`)) (`SceneComponent.K2_GetComponentRotation` (`self.Arrow`)) false true)
    (set `MovementComponent.Velocity` (* (`self.GetActorForwardVector`) (`self.Bullet_Speed`)) (`/Game/Blueprint/IA_Trashmob/BP/BP_AI_Bullet.ProjectileMovement` (`self.bullet`)))
    (`KismetSystemLibrary.K2_PauseTimerHandle` (`self.Event_Shoot`))
    (else
      (`/Engine/EditorBlueprintResources/StandardMacros.IncrementInt` (`self.NBullet`)
        (:`  `
          (`self.realoadBullet`))))))

(event `AI_Shoot`
  ;[1 0.4353 0] Shoot_Event
  (set `self.Bullet_Speed` 3500)
  (goto _label_2))

(fn `AI_Move_Forward_Function`
  (`self.AddMovementInput` (* (`KismetMathLibrary.GetForwardVector` (`self.K2_GetActorRotation`)) (`self.Speed_Multiply`))))

(fn `AI_Rotate_To_Player_Function`
  (bind _output_get (set `self.AI_New_Rotation` (`KismetMathLibrary.RInterpTo_Constant` (`self.K2_GetActorRotation`) (`KismetMathLibrary.FindLookAtRotation` (`self.K2_GetActorLocation`) (`self.K2_GetActorLocation` (`self.Player_Ref`))) (`GameplayStatics.GetWorldDeltaSeconds`) 100.0)))
  (`self.K2_SetActorRotation` _output_get))

(fn `AI_Speed_Modifier_To_Catch_Player_Function`
  ;[0 0 0] PAS TOUCHER !!!!
)

(fn `Debug_Print_Function`
  (bind _result (`/Game/Blueprint/IA_Trashmob/BP/BP_AI_Trashmob_Child.Debug_Print_Function` (`self.AI_Trashmob_Child_Ref`)))
  (`KismetSystemLibrary.PrintText` (`|FormatText` "Master AI Debug : \n \nPlayer Speed : {B} \nDistance AI To Player: {C} \nAI Speed Multiply : {D} \nE AI Movement : {E} \nAI Is In Range Of Player : {F} \nAI Wave : {G} \nAI_Distance_To_Shoot : {H} \nIs_Master : {I} \n \nChild AI Debug :  \n \n{A}" _result (`/Game/XwingPlayer/BP_Xwing.Current forward speed` (`self.Player_Ref`)) (`self.Distance_AI_To_Player`) (`self.Speed_Multiply`) (`|GetEnumeratorNameAsString` (`self.E_AI_Movement`)) (`self.AI_Is_In_Range_Of_Player`) (`|GetEnumeratorNameAsString` (`self.E_On_Change_Wave`)) (`self.AI_Distance_To_Shoot`) (`self.Is_Master_??`)) true true (struct :`R` 0.035046 :`G` 1.0 :`A` 1.0) 0.0))

(fn `Dodge_Player_Function`
  (`self.Player_Ref`
    (:`then`
      (if (`self.AI_Is_In_Range_Of_Player`)
        (set `self.PlayerSplineRef` (`self.Get_Spline_Ref_Function`))
        (set `self.E_AI_Movement` "NewEnumerator4")))
    (:`else`)))

(fn `Follow_Spline_Function`
  (bind _playersplineref (`self.PlayerSplineRef`)
    (:`then`
      (bind _output_get (set `self.SplineLocTarget` (`SplineComponent.FindLocationClosestToWorldLocation` _playersplineref (+ (`self.K2_GetActorLocation`) (* (`self.GetActorForwardVector`) 400.0)) "World")))
      (bind _output_get_2 (set `self.AI_New_Rotation` (`KismetMathLibrary.RInterpTo_Constant` (`self.K2_GetActorRotation`) (`KismetMathLibrary.FindLookAtRotation` (`self.K2_GetActorLocation`) _output_get) (`GameplayStatics.GetWorldDeltaSeconds`) 100.0)))
      (`self.K2_SetActorRotation` _output_get_2)
      (if (== (`SplineComponent.GetDistanceAlongSplineAtLocation` (`self.PlayerSplineRef`) (`self.SplineLocTarget`) "World") 0.0)
        (set `self.E_AI_Movement` "NewEnumerator1")))
    (:`else`)))

(fn `Get/Set_Distance_To_Player_Call_Shoot_Event_Function`
  ;[0.03137 1 0.949] Get/Set_Distance_Ai_To_Player
  (bind _output_get (set `self.Distance_AI_To_Player` (`self.GetDistanceTo` (`self.Player_Ref`))))
  (bind _output_get_2 (set `self.AI_Distance_To_Shoot` (`KismetMathLibrary.InRange_FloatFloat` _output_get 1500.0 6000.0)))
  (if (and _output_get_2 (not (`KismetSystemLibrary.K2_IsTimerActiveHandle` (`self.Event_Shoot`))))
    ;[0.03137 1 0.949] Call_Shoot_Event
    (bind _returnvalue (`KismetSystemLibrary.K2_SetTimerDelegate` (`|CreateDelegate` :!event `AI_Shoot`) (`self.AI_Fire_Rate`) false 0.0 (`KismetMathLibrary.RandomFloatInRange` 0.5 1.0)))
    (set `self.Event_Shoot` _returnvalue)
    (else
      (`KismetSystemLibrary.K2_PauseTimerHandle` (`self.Event_Shoot`)))))

(fn `Get_Spline_Ref_Function`
  (returns (ReturnValue :type "SplineComponent Object Reference"))
  (bind _player_ref (`self.Player_Ref`))
  (return (select `bool` (> (`KismetMathLibrary.Dot_VectorVector` (`self.GetActorForwardVector` (`self.Player_Ref`)) (`self.GetActorForwardVector`)) 0.0) :`false` (`/Game/XwingPlayer/BP_Xwing.Front_Spline` _player_ref) :`true` (`/Game/XwingPlayer/BP_Xwing.Back_Spline` _player_ref))))

(fn `Undodge_Player_Function`
  (`self.Player_Ref`
    (:`then`
      (if (not (`self.AI_Is_In_Range_Of_Player`))
        (set `self.E_AI_Movement` "NewEnumerator0")))
    (:`else`)))

(fn `UserConstructionScript`
  (bind _weakpoint_01 (`self.WeakPoint_01`))
  ;[0 0 0] Random_WeakPoint
  ;
  ; NE PAS TOUCHER
  (`SceneComponent.SetVisibility` _weakpoint_01 false false)
  (`SceneComponent.SetVisibility` (`self.WeakPoint_02`) false false)
  (`SceneComponent.SetVisibility` (`self.WeakPoint_03`) false false)
  (`PrimitiveComponent.SetCollisionEnabled` _weakpoint_01 "NoCollision")
  (`PrimitiveComponent.SetCollisionEnabled` (`self.WeakPoint_02`) "NoCollision")
  (`PrimitiveComponent.SetCollisionEnabled` (`self.WeakPoint_03`) "NoCollision")
  (`SceneComponent.SetHiddenInGame` _weakpoint_01 true false)
  (`SceneComponent.SetHiddenInGame` (`self.WeakPoint_02`) true false)
  (`SceneComponent.SetHiddenInGame` (`self.WeakPoint_03`) true false))