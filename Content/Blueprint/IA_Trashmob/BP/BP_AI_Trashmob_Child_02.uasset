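; Child trashmob enemy that turns toward the master trashmob, is built to shoot at the player's X-wing, and dies on any damage.
; Tick switches on a movement enum, starting in Debug, which only rotates; forward movement is unwired.
; Shooting reuses pooled bullets through a distance-gated timer, but BeginPlay's timer name differs from that distance function's name.
; Construction hides all three weak points, leaving random selection disconnected.
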(event `self.ReceiveBeginPlay`
  ;[0 0 0] Set_Ref_&_Variables
  (bind _returnvalue (`GameplayStatics.GetActorOfClass` "/Game/Blueprint/IA_Trashmob/BP/BP_AI_Trashmob_Master.BP_AI_Trashmob_Master_C"))
  (set `self.BP_AI_Trashmob_Master_Ref` _returnvalue)
  (bind _returnvalue_2 (`GameplayStatics.GetActorOfClass` "/Game/XwingPlayer/BP_Xwing.BP_Xwing_C"))
  (set `self.Player_Ref` _returnvalue_2)
  (bind _outactors (`GameplayStatics.GetAllActorsOfClass` "/Game/Blueprint/IA_Trashmob/BP/BP_AI_Bullet.BP_AI_Bullet_C"))
  (set `self.AI_Bullet_Ref` _outactors)
  (set `self.AI_Is_In_Range_Of_Player` false)
  (set `self.Speed_Multiply` (* (`/Game/XwingPlayer/BP_Xwing.Current forward speed` (`self.Player_Ref`)) 2.0))
  (set `self.E_AI_Child_Movement` "NewEnumerator3")
  (bind _returnvalue_3 (`KismetSystemLibrary.K2_SetTimer` null "Get/Set_Distance_To_Player/AI_Master_&_Call_Shoot_Event" 0.2 true))
  (set `self.Distance_To_Player_Timer_Event_Ref` _returnvalue_3)
  (if (not (`KismetSystemLibrary.K2_IsTimerActiveHandle` (`self.Debug_Print_Timer_Function_Ref`)))
    (bind _returnvalue_4 (`KismetSystemLibrary.K2_SetTimer` null "Debug_Print_Function" 0.015 true))
    (set `self.Debug_Print_Timer_Function_Ref` _returnvalue_4)))

(event `self.ReceiveTick`
  (params (DeltaSeconds :type "Float (single-precision)"))
  (`|ExecutionSequence`
    (:`then_0`
      ;[1 1 0] AI_Switch_Movement
      (switch `/Game/Blueprint/IA_Trashmob/BP/E_AI_Child_Movement` (`self.E_AI_Child_Movement`)
        (:`NewEnumerator4`
          (`self.Follow_Master`))
        (:`NewEnumerator3`
          (`self.AI_Child_Rotate_To_AI_Master_Function`))))))

(event `Follow_Master`
  (`KismetSystemLibrary.PrintString` "Hello")
  (bind _returnvalue (`KismetSystemLibrary.K2_SetTimer` null "AI_Child_Rotate_To_AI_Master_Function" 0.2 true))
  (set `self.AI_Child_Rotate_To_AI_Master_Function_Ref` _returnvalue))

(event `self.ReceiveAnyDamage`
  (params (Damage :type "Float (single-precision)") (DamageType :type "DamageType Object Reference") (InstigatedBy :type "Controller Object Reference") (DamageCauser :type "Actor Object Reference"))
  ;[1 0 0] Kill_AI_When_Player_Bullet_Touch_Them
  (`self.K2_DestroyActor`))

(event `self.OptimizationProxy.OnChangeWave`
  (params (NewWave :type "EOptimizationWave Enum" :default "Invisible"))
  (set `self.E_On_Change_Wave` NewWave))

(event `AI_Range_To_See_Player`
  (bind _returnvalue (`SceneComponent.K2_GetComponentLocation` (`self.AI_Trashmob`)))
  ;[1 0.4353 0] AI_Range_To_See_Player
  (bind (_outhit _returnvalue_2) (`KismetSystemLibrary.SphereTraceSingle` _returnvalue _returnvalue 5000.0 "TraceTypeQuery3"))
  (bind _output_get (set `self.AI_Is_In_Range_Of_Player` _returnvalue_2))
  (if _output_get
    (cast `/Game/XwingPlayer/BP_Xwing` (`.HitActor` (`GameplayStatics.BreakHitResult` _outhit))
      (:`CastFailed`
        _)))
  (`KismetSystemLibrary.K2_PauseTimerHandle` (`self.Event_Shoot`)))

(event `realoadBullet`
  (bind _output (`|GetArrayItem` (`self.AI_Bullet_Ref`) (`self.NBullet`)))
  ;[1 0.4353 0] Shoot_Event
  (if (not (`/Game/Blueprint/IA_Trashmob/BP/BP_AI_Bullet.isUse` _output)) :!label _label
    (bind _output_get (set `self.bullet` _output))
    (set `/Game/Blueprint/IA_Trashmob/BP/BP_AI_Bullet.isUse` true _output_get)
    (`/Game/Blueprint/IA_Trashmob/BP/BP_AI_Bullet.Spawn_Bullet_Function` _output)
    (`self.K2_SetActorLocationAndRotation` (`self.bullet`) (`SceneComponent.K2_GetComponentLocation` (`self.Arrow`)) (`SceneComponent.K2_GetComponentRotation` (`self.Arrow`)) false true)
    (set `MovementComponent.Velocity` (* (`self.GetActorForwardVector`) (`self.Bullet_Speed`)) (`/Game/Blueprint/IA_Trashmob/BP/BP_AI_Bullet.ProjectileMovement` (`self.bullet`)))
    (`KismetSystemLibrary.K2_PauseTimerHandle` (`self.Event_Shoot`))
    (else
      (`/Engine/EditorBlueprintResources/StandardMacros.IncrementInt` (`self.NBullet`)
        (:`  `
          (`self.realoadBullet`))))))

(event `AI_Shoot`
  ;[1 0.4353 0] Shoot_Event
  (set `self.Bullet_Speed` 3500)
  (goto _label))

(fn `AI_Child_Rotate_To_AI_Master_Function`
  (bind _output_get (set `self.AI_New_Rotation` (`KismetMathLibrary.RInterpTo_Constant` (`self.K2_GetActorRotation`) (`KismetMathLibrary.FindLookAtRotation` (`self.K2_GetActorLocation`) (`self.K2_GetActorLocation` (`self.BP_AI_Trashmob_Master_Ref`))) (`GameplayStatics.GetWorldDeltaSeconds`) 100.0)))
  (`self.K2_SetActorRotation` _output_get))

(fn `AI_Move_Forward_Function`
  (`self.AddMovementInput` (* (`KismetMathLibrary.GetForwardVector` (`self.K2_GetActorRotation`)) (`self.Speed_Multiply`))))

(fn `Debug_Print_Function`
  (`KismetSystemLibrary.PrintText` (`|FormatText` "AI Child Debug :  \n \nDistance AI Child To AI Master : {A} \nE AI Movement : {B} \nIs Master : {C}" (`self.Distance_AI_Child_To_AI_Master`) (`|GetEnumeratorNameAsString` (`self.E_AI_Child_Movement`)) (`self.Is_Master_??`)) true true (struct :`R` 0.035046 :`G` 1.0 :`A` 1.0) 0.0))

(fn `Get/Set_Distance_To_Player_&_Call_Shoot_Event_Function`
  ;[0.03137 1 0.949] Get/Set_Distance_Ai_To_Player
  (`|ExecutionSequence`
    (:`then_0`
      (bind _output_get (set `self.Distance_AI_To_Player` (`self.GetDistanceTo` (`self.Player_Ref`))))
      (bind _output_get_2 (set `self.AI_Distance_To_Shoot` (`KismetMathLibrary.InRange_FloatFloat` _output_get 1500.0 6000.0)))
      (if (and _output_get_2 (not (`KismetSystemLibrary.K2_IsTimerActiveHandle` (`self.Event_Shoot`))))
        ;[0.03137 1 0.949] Call_Shoot_Event
        (bind _returnvalue (`KismetSystemLibrary.K2_SetTimerDelegate` (`|CreateDelegate` :!event `AI_Shoot`) (`self.AI_Fire_Rate`) false 0.0 (`KismetMathLibrary.RandomFloatInRange` 0.5 1.0)))
        (set `self.Event_Shoot` _returnvalue)
        (else
          (`KismetSystemLibrary.K2_PauseTimerHandle` (`self.Event_Shoot`)))))
    (:`then_1`
      ;[0.03137 1 0.949] Get/Set_Distance_Ai_Child_To_Ai_Master
      (set `self.Distance_AI_Child_To_AI_Master` (`self.GetDistanceTo` (`self.BP_AI_Trashmob_Master_Ref`)))
      (if (not (`KismetMathLibrary.InRange_FloatFloat` (`self.Distance_AI_Child_To_AI_Master`) 600.0 3000.0))
        (set `self.E_AI_Child_Movement` "NewEnumerator3")))))

(fn `UserConstructionScript`
  (bind _weakpoint_01 (`self.WeakPoint_01`))
  ;[0 0 0] Random_WeakPoint
  ;
  ; NE PAS TOUCHER
  (`SceneComponent.SetVisibility` _weakpoint_01 false false)
  (`SceneComponent.SetVisibility` (`self.WeakPoint_02`) false false)
  (`SceneComponent.SetVisibility` (`self.WeakPoint_03`) false false)
  (`PrimitiveComponent.SetCollisionEnabled` _weakpoint_01 "NoCollision")
  (`PrimitiveComponent.SetCollisionEnabled` (`self.WeakPoint_02`) "NoCollision")
  (`PrimitiveComponent.SetCollisionEnabled` (`self.WeakPoint_03`) "NoCollision")
  (`SceneComponent.SetHiddenInGame` _weakpoint_01 true false)
  (`SceneComponent.SetHiddenInGame` (`self.WeakPoint_02`) true false)
  (`SceneComponent.SetHiddenInGame` (`self.WeakPoint_03`) true false))