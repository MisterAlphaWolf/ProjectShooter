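; Reusable bullet actor for the trash mob AI that applies light damage on sphere overlap and clears its in-use flag.
; It starts hidden; a spawn event turns on the sphere's visibility and collision rather than creating a new actor.
; Hiding teleports it to a disable position, disables the sphere and zeroes BulletSpeed on the first trash mob found.
; An optimization proxy also hides it on reaching the third distance wave.
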(event `self.ReceiveBeginPlay`
  ;[0 0 0] Set_Sphere_Visibility/Collision/Hide_in_Game_To_False_On_Begin_Play
  (bind _returnvalue (`GameplayStatics.GetActorOfClass` "/Game/Blueprint/IA_Trashmob/BP/BP_AI_Trashmob.BP_AI_Trashmob_C"))
  (set `self.Player_Ref` _returnvalue)
  (`self.Hide_Bullet`))

(event `self.Sphere.OnComponentBeginOverlap`
  (params (OverlappedComponent :type "PrimitiveComponent Object Reference") (OtherActor :type "Actor Object Reference") (OtherComp :type "PrimitiveComponent Object Reference") (OtherBodyIndex :type Integer) (bFromSweep :type Boolean) (SweepResult :type "HitResult Structure (by ref)"))
  ;[1 0 0] Set_Apply_Damage_On_Any_Component_Who_Hit_The_Sphere
  (`GameplayStatics.ApplyDamage` null 0.1 null self)
  (set `self.isUse` false))

(event `Spawn_Bullet`
  (bind _sphere (`self.Sphere`))
  ;[0.05725 1 0] Event_Spawn_Bullet_To_Set_Visibility/Collision/Hide_In_Game_To_True
  (`SceneComponent.SetVisibility` _sphere true false)
  (`PrimitiveComponent.SetCollisionEnabled` _sphere "QueryAndPhysics")
  (`SceneComponent.SetHiddenInGame` _sphere false false)
  (`KismetSystemLibrary.K2_PauseTimerHandle` (`self.Hide_Bullet_Timer_Ref`)))

(event `Hide_Bullet`
  (bind _sphere (`self.Sphere`))
  ;[1 1 1] Hide_Bullet_Event
  (`self.K2_SetActorLocation` (`self.Bullet_Disable_Position`) false true)
  (set `/Game/Blueprint/IA_Trashmob/BP/BP_AI_Trashmob.Bullet_Speed` 0 (`self.Player_Ref`))
  (`SceneComponent.SetVisibility` _sphere false false)
  (`PrimitiveComponent.SetCollisionEnabled` _sphere "NoCollision")
  (`SceneComponent.SetHiddenInGame` _sphere true false)
  (`KismetSystemLibrary.K2_PauseTimerHandle` (`self.Hide_Bullet_Timer_Ref`)))

(event `self.OptimizationProxy.OnChangeWave`
  (params (NewWave :type "EOptimizationWave Enum" :default "Invisible"))
  ;[1 1 1] Call_Hide_Bullet_Event_If_AI_Optmization_Distance_Is_On_The_Third_Wave
  (switch `EOptimizationWave` NewWave
    (:`ThirdWave`
      (`self.Hide_Bullet`))))

(fn `UserConstructionScript`)