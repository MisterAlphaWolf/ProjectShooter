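; Child trash-mob AI Blueprint that starts in a Follow_Master movement state and tracks its distance to a BP_AI_Trashmob_Master actor.
; BeginPlay finds the master and starts a looping timer, apparently driving Custom_Tick, in addition to the parent's Tick.
; Custom_Tick measures that distance and switches on the movement state, though no state has logic wired.
; A debug function formats the distance as text, and BeginPlay pauses the debug print timer if active.
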(event `self.ReceiveBeginPlay`
  (bind _debug_print_timer_function_ref (`self.Debug_Print_Timer_Function_Ref`))
  (`parent.ReceiveBeginPlay`)
  (set `self.E_AI_Movement` "NewEnumerator3")
  (bind _returnvalue (`GameplayStatics.GetActorOfClass` "/Game/Blueprint/IA_Trashmob/BP/BP_AI_Trashmob_Master.BP_AI_Trashmob_Master_C"))
  (set `self.BP_AI_Trashmob_Master_Ref` _returnvalue)
  (bind _returnvalue_2 (`KismetSystemLibrary.K2_SetTimerDelegate` (`|CreateDelegate` :!event `Custom_Tick`) 0.2 true))
  (set `self.Custom_Tick_Timer_Event_Ref` _returnvalue_2)
  (if (`KismetSystemLibrary.K2_IsTimerActiveHandle` _debug_print_timer_function_ref)
    (`KismetSystemLibrary.K2_PauseTimerHandle` _debug_print_timer_function_ref)))

(event `self.ReceiveTick`
  (params (DeltaSeconds :type "Float (single-precision)"))
  (`parent.ReceiveTick` DeltaSeconds))

(event `Custom_Tick`
  (`|ExecutionSequence`
    (:`then_0`
      (`self.Get_Distance_AI_Child_To_Master`))
    (:`then_1`
      (switch `/Game/Blueprint/IA_Trashmob/BP/E_AI_Movement` (`self.E_AI_Movement`)))))

(fn `Child_Debug_Function`
  (returns (Result :type Text))
  (return (`|FormatText` " \n \nDistance AI Child To AI Master : {A}" (`KismetTextLibrary.Conv_DoubleToText` (`self.Distance_AI_Child_To_Master`) "HalfToEven"))))

(fn `Get_Distance_AI_Child_To_Master`
  (set `self.Distance_AI_Child_To_Master` (`self.GetDistanceTo` (`self.BP_AI_Trashmob_Master_Ref`))))

(fn `UserConstructionScript`
  (`parent.UserConstructionScript`))