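; Pooled homing bullet for trashmob AI that deals damage to the player's X-wing.
; On BeginPlay it locks homing onto the ship's skeletal mesh, then hides itself.
; Hiding teleports it to a disable position, zeroes BulletSpeed on the first found trashmob and turns off sphere visibility and collision; a spawn function restores the sphere.
; Hitting the X-wing or entering the optimization proxy's Invisible wave hides it again.
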(event `self.ReceiveBeginPlay`
  (bind _projectilemovement (`self.ProjectileMovement`))
  ;[0 0 0] Set_Sphere_Visibility/Collision/Hide_in_Game_To_False_On_Begin_Play
  (bind _returnvalue (`GameplayStatics.GetActorOfClass` "/Game/Blueprint/XwingPlayer/BP_Xwing.BP_Xwing_C"))
  (set `self.Player_Ref` _returnvalue)
  (bind _returnvalue_2 (`GameplayStatics.GetActorOfClass` "/Game/Blueprint/IA_Trashmob/BP_AI_Trashmob_Master.BP_AI_Trashmob_Master_C"))
  (set `self.AI_Trashmob_Ref` _returnvalue_2)
  (bind _player_ref (`self.Player_Ref`)
    (:`then`
      (set `ProjectileMovementComponent.HomingTargetComponent` (`/Game/Blueprint/XwingPlayer/BP_Xwing.Ship_Skeletal_Mesh` _player_ref) _projectilemovement)
      (set `ProjectileMovementComponent.bIsHomingProjectile` true _projectilemovement)
      (`self.Hide_Bullet_Function`))
    (:`else`)))

(event `self.Sphere.OnComponentBeginOverlap`
  (params (OverlappedComponent :type "PrimitiveComponent Object Reference") (OtherActor :type "Actor Object Reference") (OtherComp :type "PrimitiveComponent Object Reference") (OtherBodyIndex :type Integer) (bFromSweep :type Boolean) (SweepResult :type "HitResult Structure (by ref)"))
  ;[1 0 0] Set_Apply_Damage_On_Any_Component_Who_Hit_The_Sphere
  (bind _asbp_xwing (cast `/Game/Blueprint/XwingPlayer/BP_Xwing` OtherActor))
  (`GameplayStatics.ApplyDamage` _asbp_xwing 0.1 null self)
  (set `self.isUse` false)
  (`self.Hide_Bullet_Function`))

(event `self.OptimizationProxy.OnChangeWave`
  (params (NewWave :type "EOptimizationWave Enum" :default "Invisible"))
  ;[1 1 1] Call_Hide_Bullet_Event_If_AI_Optmization_Distance_Is_On_The_Invisible_Wave
  (switch `EOptimizationWave` NewWave
    (:`Invisible`
      (`self.Hide_Bullet_Function`))))

(fn `Hide_Bullet_Function`
  (bind _sphere (`self.Sphere`))
  (`self.K2_SetActorLocation` (`self.Bullet_Disable_Position`) false true)
  (set `/Game/Blueprint/IA_Trashmob/BP_AI_Trashmob_Master.Bullet_Speed` 0 (`self.AI_Trashmob_Ref`))
  (`SceneComponent.SetVisibility` _sphere false false)
  (`PrimitiveComponent.SetCollisionEnabled` _sphere "NoCollision")
  (`SceneComponent.SetHiddenInGame` _sphere true false))

(fn `Spawn_Bullet_Function`
  (bind _sphere (`self.Sphere`))
  (`SceneComponent.SetVisibility` _sphere true false)
  (`PrimitiveComponent.SetCollisionEnabled` _sphere "QueryAndPhysics")
  (`SceneComponent.SetHiddenInGame` _sphere false false))

(fn `UserConstructionScript`)