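; AIC_Trashmob is the AI controller for Trashmob enemies, running the BT_Trashmob behavior tree on BeginPlay.
; Perception updates write the reported actor to the player-target blackboard key, with no effective filtering.
; Tick polls currently sighted actors and clears that key when its lookup fails, though the searched-for actor is not specified.
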(event `self.ReceiveBeginPlay`
  (`self.RunBehaviorTree` "/Game/Blueprint/IA_Trashmob/BT_Trashmob.BT_Trashmob"))

(event `self.ReceiveTick`
  (params (DeltaSeconds :type "Float (single-precision)"))
  (if (== (`KismetArrayLibrary.Array_Find` (`AIPerceptionComponent.GetCurrentlyPerceivedActors` (`self.AIPerception`) "/Script/AIModule.AISense_Sight")) -1)
    (`BlackboardComponent.SetValueAsObject` (`self.Blackboard`) (`self.Key_Player_Target`) null)))

(event `self.AIPerception.OnTargetPerceptionUpdated`
  (params (Actor :type "Actor Object Reference") (Stimulus :type "AIStimulus Structure"))
  (if true
    (`BlackboardComponent.SetValueAsObject` (`self.Blackboard`) (`self.Key_Player_Target`) Actor)))

(fn `UserConstructionScript`)