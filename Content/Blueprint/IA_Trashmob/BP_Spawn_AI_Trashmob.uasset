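; Spawner actor that creates trashmob AI (BP_AI_Trashmob_Master), either on its own or on behalf of the boss.
; Unless SpawnByBoss is set, a looping timer with a randomized interval spawns mobs at the spawner until NbrTrashmobMax is reached, then clears itself.
; AI_Spawn_By_Boss instead spawns one mob per call at a random BP_NestPatern2_Start, without checking the cap.
; Both paths set the mob's initial movement state.
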(event `self.ReceiveBeginPlay`
  ;[0 0 0] Timer_By_Event_To_Spawn_AI
  (set `self.Nbr_Of_Trashmob` 0)
  (bind _outactors (`GameplayStatics.GetAllActorsOfClass` "/Game/Blueprint/Boss/Mathieu_Boss/BP_NestPatern2_Start.BP_NestPatern2_Start_C"))
  (set `self.Nest Array ref` _outactors)
  (if (not (`self.Spawn_By_Boss`))
    (bind _returnvalue (`KismetSystemLibrary.K2_SetTimerDelegate` (`|CreateDelegate` :!event `Spawn_All_AI`) (`KismetMathLibrary.RandomFloatInRange` 1.0 2.0) true))
    (set `self.Event_SpawnAI` _returnvalue)))

(event `Spawn_All_AI`
  ;[0 1 0.5569] Spawn_AI_Event_(Only_If_The_AI_Is_Not_Spawned_By_The_Boss)
  (if (!= (`self.Nbr_Of_Trashmob`) (`self.Nbr_Trashmob_Max`))
    (bind _returnvalue (`|SpawnActorFromClass` "/Game/Blueprint/IA_Trashmob/BP_AI_Trashmob_Master.BP_AI_Trashmob_Master_C" (`KismetMathLibrary.MakeTransform` (`self.K2_GetActorLocation`)) "AdjustIfPossibleButAlwaysSpawn" "MultiplyWithRoot" null null))
    (`/Engine/EditorBlueprintResources/StandardMacros.IncrementInt` (`self.Nbr_Of_Trashmob`)
      (:`  `
        (`|VariableSetRef` (`/Game/Blueprint/IA_Trashmob/BP_AI_Trashmob_Master.E_AI_Movement` _returnvalue) "NewEnumerator0")))
    (else
      (`KismetSystemLibrary.K2_ClearAndInvalidateTimerHandle` (`self.Event_SpawnAI`)))))

(event `AI_Spawn_By_Boss`
  ;[0 0.2188 0.1218] Spawn_AI_Event_(Only_Ai_Is_Spawned_by_The_Boss)
  (bind _returnvalue (`|SpawnActorFromClass` "/Game/Blueprint/IA_Trashmob/BP_AI_Trashmob_Master.BP_AI_Trashmob_Master_C" (`KismetMathLibrary.MakeTransform` (`self.K2_GetActorLocation` (`KismetArrayLibrary.Array_Random` (`self.Nest Array ref`)))) "AdjustIfPossibleButAlwaysSpawn" "MultiplyWithRoot" null null))
  (`/Engine/EditorBlueprintResources/StandardMacros.IncrementInt` (`self.Nbr_Of_Trashmob`)
    (:`  `
      (`|VariableSetRef` (`/Game/Blueprint/IA_Trashmob/BP_AI_Trashmob_Master.E_AI_Movement` _returnvalue) "NewEnumerator0"))))

(event `self.ReceiveTick`
  (params (DeltaSeconds :type "Float (single-precision)"))
  ;[1 0 0] Debug_Nbr_Of_AI
)

(fn `UserConstructionScript`)