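; BP_BossMathis is a boss with a shielded interphase, started on BeginPlay or by the Interphase event.
; A looping timer raises the shield and spawns trashmobs through BP_Spawn_AI_Trashmob until the NBtrashmob count runs out.
; After a delay, FinInterphase drops the shield, though CanTakeDamage stays false, and the timer is cleared.
; The construction script scales the body and a larger shield from width and length variables.
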(event `self.ReceiveBeginPlay`
  (bind _shield (`self.Shield`))
  (bind _returnvalue (`GameplayStatics.GetActorOfClass` "/Game/Blueprint/IA_Trashmob/BP/BP_Spawn_AI_Trashmob.BP_Spawn_AI_Trashmob_C"))
  (set `self.Spawn trashmob ref` _returnvalue)
  (set `self.Can take damage ?` false :!label _label)
  (`SceneComponent.SetVisibility` _shield true false)
  (`PrimitiveComponent.SetCollisionEnabled` _shield "QueryAndPhysics")
  (bind _returnvalue_2 (`KismetSystemLibrary.K2_SetTimerDelegate` (delegate `Spawn Ennemi`) 0.5 true))
  (set `self.Event spawn ennemi` _returnvalue_2))

(event `Interphase`
  (goto _label))

(event `Spawn Ennemi`
  (bind _nbtrashmob (`self.NBtrashmob`))
  (if (> _nbtrashmob 0)
    (`/Engine/EditorBlueprintResources/StandardMacros.DecrementInt` _nbtrashmob
      (:`  `
        (`/Game/Blueprint/IA_Trashmob/BP/BP_Spawn_AI_Trashmob.AI_Spawn_By_Boss` (`self.Spawn trashmob ref`))))
    (else
      (`KismetSystemLibrary.Delay` (`self.Duree interphase`))
      (`self.Fin interphase`)
      (`KismetSystemLibrary.K2_ClearAndInvalidateTimerHandle` (`self.Event spawn ennemi`)))))

(event `Fin interphase`
  (bind _shield (`self.Shield`))
  (set `self.Can take damage ?` false)
  (`SceneComponent.SetVisibility` _shield false false)
  (`PrimitiveComponent.SetCollisionEnabled` _shield "NoCollision"))

(fn `UserConstructionScript`
  (bind _scale_boss_largeur (`self.Scale boss largeur`))
  (bind _scale_boss_longeur (`self.Scale boss longeur`))
  (bind _returnvalue (+ _scale_boss_largeur 5.0))
  (`SceneComponent.SetWorldScale3D` (`self.BossBody`) (`KismetMathLibrary.MakeVector` _scale_boss_largeur _scale_boss_largeur _scale_boss_longeur))
  (`SceneComponent.SetWorldScale3D` (`self.Shield`) (`KismetMathLibrary.MakeVector` _returnvalue _returnvalue (+ _scale_boss_longeur 5.0))))