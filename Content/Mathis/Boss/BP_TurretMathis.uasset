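; Boss turret that, after a short delay on begin play, rotates toward the player every tick, clamped within 45 degrees of its initial rotation per axis.
; StartShooting and StopShooting control a looping timer with randomized start variance, but Shoot is empty and the bullet spawn is disconnected.
; Dead clears the timer and makes Tick zero the rotation.
; The construction script scales the mesh from BP_BossMathis's width.
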(event `self.ReceiveBeginPlay`
  (set `self.RotationInitial` (`self.K2_GetActorRotation`))
  (`KismetSystemLibrary.Delay` 1.0)
  (set `self.CanRotate` true))

(event `self.ReceiveTick`
  (params (DeltaSeconds :type "Float (single-precision)"))
  (bind _returnvalue (`KismetMathLibrary.Conv_IntToDouble` (`KismetMathLibrary.FFloor` 0.0)))
  (bind _roll (.roll (`self.RotationInitial`)))
  (bind _pitch (.pitch (`self.RotationInitial`)))
  (bind _yaw (.yaw (`self.RotationInitial`)))
  (if (`self.CanRotate`)
    (if (`self.IsDead?`)
      (`self.K2_SetActorRotation` (`KismetMathLibrary.MakeRotator` _returnvalue _returnvalue _returnvalue))
      (else
        (`self.K2_SetActorRotation` (`KismetMathLibrary.MakeRotator` (`KismetMathLibrary.FClamp` (`KismetMathLibrary.Abs` (- _roll (.roll (`KismetMathLibrary.FindLookAtRotation` (`self.K2_GetActorLocation`) (`self.K2_GetActorLocation` (`GameplayStatics.GetPlayerPawn` 0)))))) (- _roll 45.0) (+ _roll 45.0)) (`KismetMathLibrary.FClamp` (`KismetMathLibrary.Abs` (- _pitch (.pitch (`KismetMathLibrary.FindLookAtRotation` (`self.K2_GetActorLocation`) (`self.K2_GetActorLocation` (`GameplayStatics.GetPlayerPawn` 0)))))) (- _pitch 45.0) (+ _pitch 45.0)) (`KismetMathLibrary.FClamp` (`KismetMathLibrary.Abs` (- _yaw (.yaw (`KismetMathLibrary.FindLookAtRotation` (`self.K2_GetActorLocation`) (`self.K2_GetActorLocation` (`GameplayStatics.GetPlayerPawn` 0)))))) (- _yaw 45.0) (+ _yaw 45.0))))))))

(event `StartShooting`
  (bind _returnvalue (`KismetSystemLibrary.K2_SetTimerDelegate` (`|CreateDelegate` :!event `Shoot`) 2.5 true 0.0 (`KismetMathLibrary.RandomFloatInRange` 0.25 0.75)))
  (set `self.ShootingHandle` _returnvalue))

(event `Shoot`)

(event `StopShooting`
  (`KismetSystemLibrary.K2_ClearAndInvalidateTimerHandle` (`self.ShootingHandle`)))

(event `Dead`
  (set `self.IsDead?` true)
  (`KismetSystemLibrary.K2_ClearAndInvalidateTimerHandle` (`self.ShootingHandle`)))

(fn `UserConstructionScript`
  (bind _returnvalue (`GameplayStatics.GetActorOfClass` "/Game/Mathis/Boss/BP_BossMathis.BP_BossMathis_C"))
  (bind _returnvalue_2 (/ (`/Game/Mathis/Boss/BP_BossMathis.Scale boss largeur` _returnvalue) 500.0))
  (`SceneComponent.SetWorldScale3D` (`self.StaticMesh`) (`KismetMathLibrary.MakeVector` _returnvalue_2 _returnvalue_2 _returnvalue_2)))